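; Actor that runs a WebSocket server on port 3695, turning live-stream barrage events into in-game gift effects.
; HandleMessage parses JSON into gift, chat, like, follow or join events, mapping them via Jv_PrankData save config to Normal, Box or Special triggers.
; Normal triggers go to GiftManager; Box and Special run GiftVideoPool sequences that call back into GiftManager.
; Likes accumulate toward thresholds; follows and joins fire once per username.
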(event `self.ReceiveTick`
  (params (DeltaSeconds :type "Float (single-precision)")))

(event `self.ReceiveBeginPlay`
  (bind _returnvalue (`VideoSubsystemLibrary.GetGiftVideoPool`))
  (`|ExecutionSequence`
    (:`then_0`
      (bind _returnvalue_2 (`GameplayStatics.GetActorOfClass` "/Game/PAP/BluePrint/Gift/BP_GiftManager.BP_GiftManager_C"))
      (set `self.GiftManagerRef` _returnvalue_2)
      (bind _jv_prankdata1 (`self.GetPrankData`))
      (set `self.Prank Data ` _jv_prankdata1)
      (bind _returnvalue_3 (`GameplayStatics.GetActorOfClass` "/Game/PAP/BluePrint/BP_PawnBoat.BP_PawnBoat_C"))
      (set `self.BoatRef` _returnvalue_3)
      (bind _returnvalue_4 (`GameplayStatics.GetActorOfClass` "/Game/PAP/UI/Video/BP_VideoPlayer.BP_VideoPlayer_C"))
      (set `self.VideoPlayerRef` _returnvalue_4)
      (bind _returnvalue_5 (`GameplayStatics.GetActorOfClass` "/Game/PAP/BluePrint/Manager/BP_SaveManager.BP_SaveManager_C"))
      (set `self.SaveManagerRef` _returnvalue_5))
    (:`then_1`
      (add `GiftVideoPool.OnBoxGiftLogicTrigger` _returnvalue (delegate `BoxGiftLogicTrigger`))
      (add `GiftVideoPool.OnSpecialGiftLogicTrigger` _returnvalue (delegate `SpecialGiftLogicTrigger`)))
    (:`then_2`
      (bind (_websocketserver _clientwebsocket _message) (`WebSocketListenEventsProxy.ListenAndBindEvents` (`WebSocketServer.CreateWebSocketServer`) "/*" 3695)
        (:`OnListening`
          (`KismetSystemLibrary.PrintString` "WebSocket服务启动成功"))
        (:`OnMessage`
          (`self.HandleMessage` _message))))))

(event `BoxGiftLogicTrigger`
  (params (GiftEnumValue :type Byte) (ActivateTime :type Integer) (LogicStartTimeOffset :type "Float (single-precision)") (VideoTimeInterval :type "Float (single-precision)"))
  (`/Game/PAP/BluePrint/Gift/BP_GiftManager.GiftFunCall` (`self.GiftManagerRef`) (cast `/Game/PAP/Enum/Gift_Enum` GiftEnumValue) ActivateTime LogicStartTimeOffset 0.0 VideoTimeInterval (`/Game/PAP/BluePrint/BP_PawnBoat.FinalEffectSoundVolume` (`self.BoatRef`))))

(event `SpecialGiftLogicTrigger`
  (params (GiftEnumValue :type Byte) (ActivateTime :type Integer) (LogicStartTimeOffset :type "Float (single-precision)") (VideoTimeInterval :type "Float (single-precision)"))
  (`/Game/PAP/BluePrint/Gift/BP_GiftManager.GiftFunCall` (`self.GiftManagerRef`) (cast `/Game/PAP/Enum/Gift_Enum` GiftEnumValue) ActivateTime LogicStartTimeOffset 0.0 VideoTimeInterval (`/Game/PAP/BluePrint/BP_PawnBoat.FinalEffectSoundVolume` (`self.BoatRef`))))

(event `BoxTrigger`
  (params (GiftEnums :type "Array of /Game/PAP/Enum/Gift_Enum Enum") (LogicStartoffset :type "Array of Float (double-precision)") (Interval :type "Float (double-precision)") (RandomTimes :type Integer) (AnimName :type String)))

(event `BoxDelay1`)

(event `BoxDelay2`)

(event `SpecialTrigger`
  (params (GiftEnums :type "Array of /Game/PAP/Enum/Gift_Enum Enum") (LogicStartOffset :type "Array of Float (double-precision)") (Interval :type "Float (double-precision)") (TriggerTime :type Integer) (AnimName :type String))
  (bind _newlocalvar_11 (`self.Play Special IntorVideo` AnimName))
  (bind _returnvalue (`KismetSystemLibrary.K2_SetTimerDelegate` (delegate `SpecialDelay1`) _newlocalvar_11)))

(event `SpecialDelay1`
  (`KismetSystemLibrary.K2_ClearAndInvalidateTimerHandle` (stale `SpecialTrigger` _returnvalue)))

(event `SpecialDelay2`)

(fn `GetPrankData`
  (returns (Jv_PrankData1 :type "/Game/Barrage/Jv_PrankData Object Reference"))
  (locals (Jv_PrankData :type "/Game/Barrage/Jv_PrankData Object Reference"))
  (bind _returnvalue (`GameplayStatics.DoesSaveGameExist` "Jv_PrankData"))
  (if _returnvalue
    (bind _returnvalue_2 (`GameplayStatics.LoadGameFromSlot` "Jv_PrankData"))
    (bind _asjv_prank_data (cast `/Game/Barrage/Jv_PrankData` _returnvalue_2))
    (set `local.Jv_PrankData` _asjv_prank_data)
    (else
      (bind _returnvalue_3 (`GameplayStatics.CreateSaveGameObject` "/Game/Barrage/Jv_PrankData.Jv_PrankData_C"))
      (bind _output_get (set `local.Jv_PrankData` _returnvalue_3))
      (`GameplayStatics.SaveGameToSlot` _output_get "Jv_PrankData")))
  (return (`local.Jv_PrankData`)))

(fn `HandleMessage`
  (params (Message :type String))
  (locals (`UserName-Follow` :type "Array of String") (`UserName-Join` :type "Array of String") (TotalEffectSound :type "Float (double-precision)" :default 0.0))
  (bind _returnvalue (`VideoSubsystemLibrary.GetGiftVideoPool`))
  (bind _returnvalue_2 (`VideoSubsystemLibrary.GetGiftVideoPool`))
  (bind _returnvalue_3 (`VideoSubsystemLibrary.GetGiftVideoPool`))
  (bind (_barragedata_type _barragedata_username _barragedata_avatar _barragedata_message) (break `/Game/Barrage/Structures/BarrageData` (`self.BarrageData`)))
  (bind ((`Type_2_8A9789414546527AB4219E9CD91D931E` _type) (`Message_16_98AD17CE4084AF9587AE2CB8882F0DD2` _message)) (break `/Game/Barrage/Structures/BarrageData` (`self.BarrageData`)))
  (bind ((`LikeCount_13_7D30B0934A5E587386E5BF91C7F9EB46` _likecount)) (break `/Game/Barrage/Structures/BarrageData` (`self.BarrageData`)))
  (bind ((`UserName_5_6D45E1C34A777EA642802695D884DEB4` _username)) (break `/Game/Barrage/Structures/BarrageData` (`self.BarrageData`)))
  (bind ((`UserName_5_6D45E1C34A777EA642802695D884DEB4` _username_2)) (break `/Game/Barrage/Structures/BarrageData` (`self.BarrageData`)))
  (bind _outjsonobject (`JsonBlueprintFunctionLibrary.FromString` Message))
  (set `self.Json Object` _outjsonobject)
  (`|ExecutionSequence`
    (:`then_0`
      (bind _outvalue (`|GetJsonField` (`self.Json Object`) "name"))
      (setmembers `/Game/Barrage/Structures/BarrageData` :`StructRef` (`self.BarrageData`) :`UserName` _outvalue))
    (:`then_1`
      (bind _outvalue_2 (`|GetJsonField` (`self.Json Object`) "userAvatar"))
      (setmembers `/Game/Barrage/Structures/BarrageData` :`StructRef` (`self.BarrageData`) :`Avatar` _outvalue_2))
    (:`then_2`
      (bind _outvalue_3 (`|GetJsonField` (`self.Json Object`) "message"))
      (setmembers `/Game/Barrage/Structures/BarrageData` :`StructRef` (`self.BarrageData`) :`Message` _outvalue_3))
    (:`then_3`
      (bind _outvalue_4 (`|GetJsonField` (`self.Json Object`) "num"))
      (setmembers `/Game/Barrage/Structures/BarrageData` :`StructRef` (`self.BarrageData`) :`GiftCount` _outvalue_4))
    (:`then_4`
      (bind _outvalue_5 (`|GetJsonField` (`self.Json Object`) "count"))
      (setmembers `/Game/Barrage/Structures/BarrageData` :`StructRef` (`self.BarrageData`) :`LikeCount` _outvalue_5))
    (:`then_5`
      (bind _outvalue_6 (`|GetJsonField` (`self.Json Object`) "Type"))
      (switch `string` _outvalue_6
        (:`进场`
          (set `self.Type` "NewEnumerator0"))
        (:`聊天`
          (set `self.Type` "NewEnumerator2"))
        (:`礼物`
          (set `self.Type` "NewEnumerator1"))
        (:`关注`
          (set `self.Type` "NewEnumerator4"))
        (:`点赞`
          (set `self.Type` "NewEnumerator3")))
      (setmembers `/Game/Barrage/Structures/BarrageData` :`StructRef` (`self.BarrageData`) :`Type` (`self.Type`))
      (bind _jv_prankdata1 (`self.GetPrankData`))
      (set `self.Prank Data ` _jv_prankdata1)
      (bind _returntotal___effectmusic (`/Game/PAP/BluePrint/Manager/BP_SaveManager.GetEffectMusic` (`self.SaveManagerRef`)))
      (set `local.TotalEffectSound` _returntotal___effectmusic)
      (switch `/Game/Barrage/Enums/BarrageType` (`.Type_2_8A9789414546527AB4219E9CD91D931E` (break `/Game/Barrage/Structures/BarrageData` (`self.BarrageData`)))
        (:`NewEnumerator1`
          (`KismetSystemLibrary.PrintString` (`KismetStringLibrary.Concat_StrStr` "Gift : " _barragedata_message) true true (struct :`R` 0.344864 :`G` 1.0 :`B` 0.196227 :`A` 1.0) 0.5)
          ;[1 1 1] 礼物触发区
          (bind (_return _intervaltime1 _gifttriggertype1 _randomtimes1 _animname1) (`/Game/PAP/BluePrint/Gift/BP_GiftManager.Message to Gift Name` (`self.GiftManagerRef`) _message (`self.Prank Data `) _type :!label _label))
          (bind _newparam1 (`self.StringsToTextes` _return))
          (bind (_giftnameenums1 _logicstartdelaytimes1) (`/Game/PAP/BluePrint/Gift/BP_GiftManager.GiftsTypeJugement` (`self.GiftManagerRef`) _newparam1))
          (switch `string` _gifttriggertype1
            (:`Normal`
              (bind _returnvalue_4 (* _randomtimes1 (`.GiftCount_11_D1E846E846D3FFA7AEF587A6E1489772` (break `/Game/Barrage/Structures/BarrageData` (`self.BarrageData`)))))
              (`/Game/PAP/BluePrint/Gift/BP_GiftManager.Video Play Called in Web` (`self.GiftManagerRef`) _giftnameenums1 _logicstartdelaytimes1 _returnvalue_4 _intervaltime1))
            (:`Box`
              (`GiftVideoPool.PlayBoxTriggerSequence` _returnvalue _giftnameenums1 _logicstartdelaytimes1 _intervaltime1 _returnvalue_4 _animname1 (`local.TotalEffectSound`) (`self.VideoPlayerRef`)))
            (:`Special`
              (`GiftVideoPool.PlaySpecialTriggerSequence` _returnvalue _giftnameenums1 _logicstartdelaytimes1 _intervaltime1 _returnvalue_4 _animname1 (`local.TotalEffectSound`) (`self.VideoPlayerRef`)))))
        (:`NewEnumerator2`
          (goto _label))
        (:`NewEnumerator3`
          (set `self.Likes` (+ (`self.Likes`) _likecount))
          (`KismetSystemLibrary.PrintString` (`KismetStringLibrary.Concat_StrStr` "Likes + :" (`KismetStringLibrary.Conv_IntToString` _likecount)))
          (bind (_returnname1 _gifttriggertype1_2 _intervaltime1_2 _triggertimes1 _animname1_2) (`self.Like Gift Trigger`))
          (bind _newparam1_2 (`self.StringsToTextes` _returnname1))
          (bind (_giftnameenums1_2 _logicstartdelaytimes1_2) (`/Game/PAP/BluePrint/Gift/BP_GiftManager.GiftsTypeJugement` (`self.GiftManagerRef`) _newparam1_2))
          (switch `string` _gifttriggertype1_2
            (:`Normal`
              (`/Game/PAP/BluePrint/Gift/BP_GiftManager.Video Play Called in Web` (`self.GiftManagerRef`) _giftnameenums1_2 _logicstartdelaytimes1_2 _triggertimes1 _intervaltime1_2))
            (:`Box`
              (`GiftVideoPool.PlayBoxTriggerSequence` _returnvalue_3 _giftnameenums1_2 _logicstartdelaytimes1_2 _intervaltime1_2 _triggertimes1 _animname1_2 (`local.TotalEffectSound`) (`self.VideoPlayerRef`)))
            (:`Special`
              (`GiftVideoPool.PlaySpecialTriggerSequence` _returnvalue_3 _giftnameenums1_2 _logicstartdelaytimes1_2 _intervaltime1_2 _triggertimes1 _animname1_2 (`local.TotalEffectSound`) (`self.VideoPlayerRef`)))))
        (:`NewEnumerator4`
          (if (not (`KismetArrayLibrary.Array_Contains` (`local.UserName-Follow`) _username))
            (`KismetArrayLibrary.Array_Add` (`local.UserName-Follow`) _username)
            (bind (_returnname1_2 _gifttriggertype1_3 _intervaltime1_3 _triggertimes1_2 _animname1_3) (`self.Join_Follow GiftLogic Find` (`.Type_2_8A9789414546527AB4219E9CD91D931E` (break `/Game/Barrage/Structures/BarrageData` (`self.BarrageData`))) :!label _label_2))
            (bind _newparam1_3 (`self.StringsToTextes` _returnname1_2))
            (bind (_giftnameenums1_3 _logicstartdelaytimes1_3) (`/Game/PAP/BluePrint/Gift/BP_GiftManager.GiftsTypeJugement` (`self.GiftManagerRef`) _newparam1_3))
            (switch `string` _gifttriggertype1_3
              (:`Normal`
                (`/Game/PAP/BluePrint/Gift/BP_GiftManager.Video Play Called in Web` (`self.GiftManagerRef`) _giftnameenums1_3 _logicstartdelaytimes1_3 _triggertimes1_2 _intervaltime1_3))
              (:`Box`
                (`GiftVideoPool.PlayBoxTriggerSequence` _returnvalue_2 _giftnameenums1_3 _logicstartdelaytimes1_3 _intervaltime1_3 _triggertimes1_2 _animname1_3 (`local.TotalEffectSound`) (`self.VideoPlayerRef`)))
              (:`Special`
                (`GiftVideoPool.PlaySpecialTriggerSequence` _returnvalue_2 _giftnameenums1_3 _logicstartdelaytimes1_3 _intervaltime1_3 _triggertimes1_2 _animname1_3 (`local.TotalEffectSound`) (`self.VideoPlayerRef`))))))
        (:`NewEnumerator0`
          (if (not (`KismetArrayLibrary.Array_Contains` (`local.UserName-Join`) _username_2))
            (`KismetArrayLibrary.Array_Add` (`local.UserName-Join`) _username_2)
            (goto _label_2)))))))

(fn `Join_Follow GiftLogic Find`
  (params (Type :type "/Game/Barrage/Enums/BarrageType Enum" :default "NewEnumerator1"))
  (returns (ReturnName1 :type "Array of String") (GiftTriggerType1 :type String) (IntervalTime1 :type "Float (double-precision)") (TriggerTimes1 :type Integer) (AnimName1 :type String))
  (locals (ReturnName :type "Array of String") (IntervalTime :type "Float (double-precision)") (TriggerTimes :type Integer) (AnimName :type String) (GiftTriggerType :type String))
  (`|ExecutionSequence`
    (:`then_0`
      (for _array_element (`/Game/Barrage/Jv_PrankData.NormalConfig` (`self.Prank Data `))
        (if (`|EnumEquality` (`.BarrageType_10_50FD620748A5087167B10C9C7954196E` (break `/Game/Barrage/Structures/PrankData` _array_element)) (`self.Type`))
          (bind ((`CallName_21_CCCAFAC546C91FAC2656FB80151D7472` _callname) (`Count_17_01DF748C4E4C119D19EB2C88D53C343D` _count) (`Delay_20_6C7844CF4DD6D17745A3A8AA9C29E67D` _delay)) (break `/Game/Barrage/Structures/PrankData` _array_element))
          (set `local.ReturnName` _callname)
          (set `local.IntervalTime` _delay)
          (set `local.TriggerTimes` _count)
          (set `local.GiftTriggerType` "Normal")
          (return (`local.ReturnName`) (`local.GiftTriggerType`) (`local.IntervalTime`) (`local.TriggerTimes`) (`local.AnimName`)))))
    (:`then_1`
      (for _array_element_2 (`/Game/Barrage/Jv_PrankData.BoxConfig` (`self.Prank Data `))
        (if (`|EnumEquality` (`.BarrageType_10_50FD620748A5087167B10C9C7954196E` (break `/Game/Barrage/Structures/PrankData` _array_element_2)) (`self.Type`))
          (bind ((`CallName_21_CCCAFAC546C91FAC2656FB80151D7472` _callname_2) (`Count_17_01DF748C4E4C119D19EB2C88D53C343D` _count_2) (`Delay_20_6C7844CF4DD6D17745A3A8AA9C29E67D` _delay_2) (`AnimName_26_21CB5A6143DE77E9F43633BBE0B257E2` _animname)) (break `/Game/Barrage/Structures/PrankData` _array_element_2))
          (set `local.ReturnName` _callname_2)
          (set `local.IntervalTime` _delay_2)
          (set `local.TriggerTimes` _count_2)
          (set `local.AnimName` _animname)
          (set `local.GiftTriggerType` "Box")
          (return (`local.ReturnName`) (`local.GiftTriggerType`) (`local.IntervalTime`) (`local.TriggerTimes`) (`local.AnimName`)))))
    (:`then_2`
      (for _array_element_3 (`/Game/Barrage/Jv_PrankData.SpecailConfig` (`self.Prank Data `))
        (if (`|EnumEquality` (`.BarrageType_10_50FD620748A5087167B10C9C7954196E` (break `/Game/Barrage/Structures/PrankData` _array_element_3)) (`self.Type`))
          (bind ((`CallName_21_CCCAFAC546C91FAC2656FB80151D7472` _callname_3) (`Count_17_01DF748C4E4C119D19EB2C88D53C343D` _count_3) (`Delay_20_6C7844CF4DD6D17745A3A8AA9C29E67D` _delay_3) (`AnimName_26_21CB5A6143DE77E9F43633BBE0B257E2` _animname_2)) (break `/Game/Barrage/Structures/PrankData` _array_element_3))
          (set `local.ReturnName` _callname_3)
          (set `local.IntervalTime` _delay_3)
          (set `local.TriggerTimes` _count_3)
          (set `local.AnimName` _animname_2)
          (set `local.GiftTriggerType` "Special")
          (return (`local.ReturnName`) (`local.GiftTriggerType`) (`local.IntervalTime`) (`local.TriggerTimes`) (`local.AnimName`)))))))

(fn `Like Gift Trigger`
  (returns (ReturnName1 :type "Array of String") (GiftTriggerType1 :type String) (IntervalTime1 :type "Float (double-precision)") (TriggerTimes1 :type Integer) (AnimName1 :type String))
  (locals (MinusNum :type Integer) (ReturnName :type "Array of String") (IntervalTime :type "Float (double-precision)") (TriggerTimes :type Integer :default 1) (GiftTriggerType :type String) (AnimName :type String))
  (`|ExecutionSequence`
    (:`then_0`
      (for _array_element (`/Game/Barrage/Jv_PrankData.NormalConfig` (`self.Prank Data `))
        (if (`|EnumEquality` (`.BarrageType_10_50FD620748A5087167B10C9C7954196E` (break `/Game/Barrage/Structures/PrankData` _array_element)) (`self.Type`))
          (bind _output_get (set `local.MinusNum` (`KismetStringLibrary.Conv_StringToInt` (`.Message_12_70B693804961B130751B50A1C9710C52` (break `/Game/Barrage/Structures/PrankData` _array_element)))))
          (if (> (`self.Likes`) _output_get)
            (set `self.Likes` (- (`self.Likes`) (`local.MinusNum`)))
            (bind ((`CallName_21_CCCAFAC546C91FAC2656FB80151D7472` _callname) (`Count_17_01DF748C4E4C119D19EB2C88D53C343D` _count) (`Delay_20_6C7844CF4DD6D17745A3A8AA9C29E67D` _delay)) (break `/Game/Barrage/Structures/PrankData` _array_element))
            (set `local.ReturnName` _callname)
            (set `local.IntervalTime` _delay)
            (set `local.TriggerTimes` _count)
            (set `local.GiftTriggerType` "Normal")
            (return (`local.ReturnName`) (`local.GiftTriggerType`) (`local.IntervalTime`) (`local.TriggerTimes`) (`local.AnimName`))))))
    (:`then_1`
      (for _array_element_2 (`/Game/Barrage/Jv_PrankData.BoxConfig` (`self.Prank Data `))
        (if (`|EnumEquality` (`.BarrageType_10_50FD620748A5087167B10C9C7954196E` (break `/Game/Barrage/Structures/PrankData` _array_element_2)) (`self.Type`))
          (bind _output_get_2 (set `local.MinusNum` (`KismetStringLibrary.Conv_StringToInt` (`.Message_12_70B693804961B130751B50A1C9710C52` (break `/Game/Barrage/Structures/PrankData` _array_element_2)))))
          (if (> (`self.Likes`) _output_get_2)
            (set `self.Likes` (- (`self.Likes`) (`local.MinusNum`)))
            (bind ((`CallName_21_CCCAFAC546C91FAC2656FB80151D7472` _callname_2) (`Count_17_01DF748C4E4C119D19EB2C88D53C343D` _count_2) (`Delay_20_6C7844CF4DD6D17745A3A8AA9C29E67D` _delay_2) (`AnimName_26_21CB5A6143DE77E9F43633BBE0B257E2` _animname)) (break `/Game/Barrage/Structures/PrankData` _array_element_2))
            (set `local.ReturnName` _callname_2)
            (set `local.IntervalTime` _delay_2)
            (set `local.TriggerTimes` _count_2)
            (set `local.AnimName` _animname)
            (set `local.GiftTriggerType` "Box")
            (return (`local.ReturnName`) (`local.GiftTriggerType`) (`local.IntervalTime`) (`local.TriggerTimes`) (`local.AnimName`))))))
    (:`then_2`
      (for _array_element_3 (`/Game/Barrage/Jv_PrankData.SpecailConfig` (`self.Prank Data `))
        (if (`|EnumEquality` (`.BarrageType_10_50FD620748A5087167B10C9C7954196E` (break `/Game/Barrage/Structures/PrankData` _array_element_3)) (`self.Type`))
          (bind _output_get_3 (set `local.MinusNum` (`KismetStringLibrary.Conv_StringToInt` (`.Message_12_70B693804961B130751B50A1C9710C52` (break `/Game/Barrage/Structures/PrankData` _array_element_3)))))
          (if (> (`self.Likes`) _output_get_3)
            (set `self.Likes` (- (`self.Likes`) (`local.MinusNum`)))
            (bind ((`CallName_21_CCCAFAC546C91FAC2656FB80151D7472` _callname_3) (`Count_17_01DF748C4E4C119D19EB2C88D53C343D` _count_3) (`Delay_20_6C7844CF4DD6D17745A3A8AA9C29E67D` _delay_3) (`AnimName_26_21CB5A6143DE77E9F43633BBE0B257E2` _animname_2)) (break `/Game/Barrage/Structures/PrankData` _array_element_3))
            (set `local.ReturnName` _callname_3)
            (set `local.IntervalTime` _delay_3)
            (set `local.TriggerTimes` _count_3)
            (set `local.AnimName` _animname_2)
            (set `local.GiftTriggerType` "Special")
            (return (`local.ReturnName`) (`local.GiftTriggerType`) (`local.IntervalTime`) (`local.TriggerTimes`) (`local.AnimName`))))))))

(fn `Play Box Intro Video`
  (params (IntroVideo :type String))
  (returns (DelayTime2 :type "Float (double-precision)"))
  (locals (DelayTime1 :type "Float (double-precision)") (GiftName :type "/Game/PAP/Enum/Gift_Enum Enum"))
  (bind _giftname (`local.GiftName`))
  (bind _introvideo (`local.IntroVideo`))
  (if (`KismetStringLibrary.EqualEqual_StrStr` _introvideo)
    _
    (elif (`KismetStringLibrary.EqualEqual_StrStr` _introvideo "盲盒1")
      (set `local.DelayTime1` 2.0)
      (set `local.GiftName` "NewEnumerator36")
      (`/Game/PAP/BluePrint/Gift/BP_GiftManager.GiftFunCall` (`self.GiftManagerRef`) _giftname 1 0.0 0.0 0.0 (`/Game/PAP/BluePrint/BP_PawnBoat.FinalEffectSoundVolume` (`self.BoatRef`)) :!label _label)
      (`KismetSystemLibrary.PrintString` (`KismetStringLibrary.Concat_StrStr` "BoxIntro ： " (`|GetEnumeratorNameAsString` _giftname)) true true (struct :`R` 0.423529 :`G` 1.0 :`B` 0.360784 :`A` 1.0) 1.0)
      (return (`local.DelayTime1`))
      (elif (`KismetStringLibrary.EqualEqual_StrStr` _introvideo "盲盒2")
        (set `local.DelayTime1` 2.0)
        (set `local.GiftName` "NewEnumerator37")
        (goto _label)
        (elif (`KismetStringLibrary.EqualEqual_StrStr` _introvideo "盲盒3")
          (set `local.DelayTime1` 2.0)
          (set `local.GiftName` "NewEnumerator38")
          (goto _label)
          (elif (`KismetStringLibrary.EqualEqual_StrStr` _introvideo "盲盒4")
            (set `local.DelayTime1` 2.0)
            (set `local.GiftName` "NewEnumerator39")
            (goto _label)))))))

(fn `Play Special IntorVideo`
  (params (`In VideoName` :type String))
  (returns (NewLocalVar_11 :type "Float (double-precision)"))
  (locals (NewLocalVar_1 :type "Float (double-precision)") (NewLocalVar :type "/Game/PAP/Enum/Gift_Enum Enum"))
  (bind _in_videoname (`local.In VideoName`))
  (if (`KismetStringLibrary.EqualEqual_StrStr` _in_videoname)
    _
    (elif (`KismetStringLibrary.EqualEqual_StrStr` _in_videoname "火力全开")
      (set `local.NewLocalVar_1` 3.0)
      (bind _output_get (set `local.NewLocalVar` "NewEnumerator40"))
      (`/Game/PAP/BluePrint/Gift/BP_GiftManager.GiftFunCall` (`self.GiftManagerRef`) _output_get 1 0.0 0.0 0.0 (`/Game/PAP/BluePrint/BP_PawnBoat.FinalEffectSoundVolume` (`self.BoatRef`)))
      (`KismetSystemLibrary.PrintString` (`KismetStringLibrary.Concat_StrStr` "SpecialIntro ： " (`|GetEnumeratorNameAsString` _output_get)) true true (struct :`R` 1.0 :`G` 0.447059 :`B` 0.415686 :`A` 1.0) 1.0)
      (return (`local.NewLocalVar_1`)))))

(fn `StringsToTextes`
  (params (NewParam :type "Array of String"))
  (returns (NewParam1 :type "Array of Text"))
  (locals (NewLocalVar :type "Array of Text"))
  (for _array_element NewParam
    (`KismetArrayLibrary.Array_Add` (`local.NewLocalVar`) (`KismetTextLibrary.Conv_StringToText` _array_element)))
  (return (`local.NewLocalVar`)))

(fn `UserConstructionScript`)