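; Cartoony FX rocket actor that prints a 3-2-1 countdown on BeginPlay and then launches upward.
; An ENUMRocketType switch (Slow, Fast, Blobby, Space) sets animation speed, effect timing and the timeline that ramps MoveSpeed.
; Tick adds MoveSpeed to the actor's Z after liftoff while keeping both RocketStart effects at fixed world heights.
; Timelines drive lens flare billboard opacity through dynamic materials; the rocket and flares are hidden shortly after launch.
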(event `self.ReceiveTick`
  (params (DeltaSeconds :type "Float (single-precision)"))
  (if (`self.IsLiftOff`)
    (`self.Move Rocket Upward`)))

(event `Move Rocket Upward`
  (bind (_returnvalue_x _returnvalue_y _returnvalue_z) (`KismetMathLibrary.BreakVector` (`self.K2_GetActorLocation`)))
  (bind _rocketstart (`self.RocketStart`))
  (bind _rocketstart2 (`self.RocketStart2`))
  (bind (_returnvalue_x_2 _returnvalue_y_2) (`KismetMathLibrary.BreakVector` (`SceneComponent.K2_GetComponentLocation` _rocketstart)))
  (bind (_returnvalue_x_3 _returnvalue_y_3) (`KismetMathLibrary.BreakVector` (`SceneComponent.K2_GetComponentLocation` _rocketstart2)))
  (`self.K2_SetActorLocation` (`KismetMathLibrary.MakeVector` _returnvalue_x _returnvalue_y (+ _returnvalue_z (`self.moveSpeed`))))
  (`SceneComponent.K2_SetWorldLocation` _rocketstart (`KismetMathLibrary.MakeVector` _returnvalue_x_2 _returnvalue_y_2 40.0) false false)
  (`SceneComponent.K2_SetWorldLocation` _rocketstart2 (`KismetMathLibrary.MakeVector` _returnvalue_x_3 _returnvalue_y_3 0.0) false false))

(event `self.ReceiveBeginPlay`
  (bind _materialbillboard1 (`self.MaterialBillboard1`))
  (bind _materialbillboard (`self.MaterialBillboard`))
  (bind _rocket (`self.Rocket`))
  (bind _rocket_2 (`self.Rocket`))
  (bind _rocket_3 (`self.Rocket`))
  (bind _rocket_4 (`self.Rocket`))
  (`KismetSystemLibrary.Delay` 1.0)
  (`KismetSystemLibrary.PrintString` "3" true true (struct :`G` 0.66 :`B` 1.0 :`A` 1.0) 1.0)
  (`KismetSystemLibrary.Delay` 1.0)
  (`KismetSystemLibrary.PrintString` "2" true true (struct :`G` 0.66 :`B` 1.0 :`A` 1.0) 1.0)
  (`KismetSystemLibrary.Delay` 1.0)
  (`KismetSystemLibrary.PrintString` "1" true true (struct :`G` 0.66 :`B` 1.0 :`A` 1.0) 1.0)
  (`KismetSystemLibrary.Delay` 1.0)
  (`KismetSystemLibrary.PrintString` "LiftOff" true true (struct :`G` 0.66 :`B` 1.0 :`A` 1.0) 1.0)
  (`|ExecutionSequence`
    (:`then_0`
      (switch `/Game/PAP/Special_Effect/CartoonyFXPACK4/Blueprints/ENUM_RocketType` (`self.ENUM_RocketType`)
        (:`NewEnumerator0`
          (`SkeletalMeshComponent.SetAnimation` _rocket_3 "/Game/PAP/Special_Effect/CartoonyFXPACK4/Meshes/ANIM_Rocket_LiftOff_Anim.ANIM_Rocket_LiftOff_Anim")
          (`SkeletalMeshComponent.SetPlayRate` _rocket_3 0.7)
          (`SkeletalMeshComponent.Play` _rocket_3 false)
          (`KismetSystemLibrary.Delay` 0.4)
          (set `self.IsLiftOff` true)
          (`SceneComponent.SetVisibility` (`self.RocketliftOff`) true false)
          (`ActorComponent.SetActive` (`self.RocketStart2`) true false)
          (`ActorComponent.SetActive` (`self.RocketStart`) false false)
          (`KismetSystemLibrary.Delay` 2.0)
          (`SceneComponent.SetVisibility` (`self.MaterialBillboard`) true false)
          (`SceneComponent.SetVisibility` (`self.MaterialBillboard1`) true false)
          (`|ExecutionSequence`
            (:`then_0`
              (bind (_direction _newtrack_0) (`Timeline|Timeline_0` :!via `PlayFromStart`)
                (:`Update`
                  (set `self.moveSpeed` (`KismetMathLibrary.Lerp` 0.3 3.0 _newtrack_0)))))
            (:`then_1`
              (`KismetSystemLibrary.Delay` 2.0)
              (`KismetSystemLibrary.Delay` 2.0)
              (`ActorComponent.SetActive` (`self.RocketStart2`) false false))))
        (:`NewEnumerator1`
          (`SkeletalMeshComponent.SetAnimation` _rocket_4 "/Game/PAP/Special_Effect/CartoonyFXPACK4/Meshes/ANIM_Rocket_LiftOff_Anim.ANIM_Rocket_LiftOff_Anim")
          (`SkeletalMeshComponent.SetPlayRate` _rocket_4 2.0)
          (`SkeletalMeshComponent.Play` _rocket_4 false)
          (`KismetSystemLibrary.Delay` 0.2)
          (set `self.IsLiftOff` true)
          (`SceneComponent.SetVisibility` (`self.RocketliftOff`) true false)
          (`ActorComponent.SetActive` (`self.RocketStart2`) true false)
          (`ActorComponent.SetActive` (`self.RocketStart`) false false)
          (`SceneComponent.SetVisibility` (`self.MaterialBillboard`) true false)
          (`SceneComponent.SetVisibility` (`self.MaterialBillboard1`) true false)
          (`|ExecutionSequence`
            (:`then_0`
              (bind (_direction_2 _newtrack_0_2) (`Timeline|Timeline_1` :!via `PlayFromStart`)
                (:`Update`
                  (set `self.moveSpeed` (`KismetMathLibrary.Lerp` 1.0 2000.0 _newtrack_0_2)))))
            (:`then_1`
              (`KismetSystemLibrary.Delay` 1.0)
              (`ActorComponent.SetActive` (`self.RocketStart2`) false false))))
        (:`NewEnumerator2`
          (`SkeletalMeshComponent.SetAnimation` _rocket_2 "/Game/PAP/Special_Effect/CartoonyFXPACK4/Meshes/ANIM_Rocket_LiftOff_Anim.ANIM_Rocket_LiftOff_Anim")
          (`SkeletalMeshComponent.SetPlayRate` _rocket_2 2.0)
          (`SkeletalMeshComponent.Play` _rocket_2 false)
          (`ActorComponent.SetActive` (`self.RocketStart2`) true false)
          (`KismetSystemLibrary.Delay` 0.2)
          (set `self.IsLiftOff` true)
          (`SceneComponent.SetVisibility` (`self.RocketliftOff`) true false)
          (`ActorComponent.SetActive` (`self.RocketStart`) false false)
          (`SceneComponent.SetVisibility` (`self.MaterialBillboard`) true false)
          (`SceneComponent.SetVisibility` (`self.MaterialBillboard1`) true false)
          (`|ExecutionSequence`
            (:`then_0`
              (`KismetSystemLibrary.Delay` 0.2)
              (bind (_direction_3 _newtrack_0_3) (`Timeline|Timeline_2` :!via `PlayFromStart`)
                (:`Update`
                  (set `self.moveSpeed` (`KismetMathLibrary.Lerp` 1.0 2000.0 _newtrack_0_3)))))
            (:`then_2`
              (`KismetSystemLibrary.Delay` 2.0)
              (`ActorComponent.SetActive` (`self.RocketStart2`) false false))))
        (:`NewEnumerator3`
          (`SkeletalMeshComponent.SetAnimation` _rocket "/Game/PAP/Special_Effect/CartoonyFXPACK4/Meshes/ANIM_Rocket_LiftOff_Anim.ANIM_Rocket_LiftOff_Anim")
          (`SkeletalMeshComponent.SetPlayRate` _rocket 2.0)
          (`SkeletalMeshComponent.Play` _rocket false)
          (`ActorComponent.SetActive` (`self.RocketStart2`) true false)
          (`KismetSystemLibrary.Delay` 0.2)
          (set `self.IsLiftOff` true)
          (`SceneComponent.SetVisibility` (`self.RocketliftOff`) true false)
          (`ActorComponent.SetActive` (`self.RocketStart`) false false)
          (`SceneComponent.SetVisibility` (`self.MaterialBillboard`) true false)
          (`SceneComponent.SetVisibility` (`self.MaterialBillboard1`) true false)
          (`|ExecutionSequence`
            (:`then_0`
              (`KismetSystemLibrary.Delay` 0.2)
              (bind (_direction_4 _newtrack_0_4) (`Timeline|Timeline_4` :!via `PlayFromStart`)
                (:`Update`
                  (set `self.moveSpeed` (`KismetMathLibrary.Lerp` 1.0 2000.0 _newtrack_0_4)))))
            (:`then_2`
              (`KismetSystemLibrary.Delay` 2.0)
              (`ActorComponent.SetActive` (`self.RocketStart2`) false false))))))
    (:`then_1`
      ;[1 1 1] Lens Flare
      (`KismetSystemLibrary.Delay` 0.3)
      (`SceneComponent.SetVisibility` _materialbillboard true false)
      (bind _returnvalue (`PrimitiveComponent.CreateDynamicMaterialInstance` _materialbillboard 0 (`.Material` (break `MaterialSpriteElement` (`|GetArrayItem` (`MaterialBillboardComponent.Elements` _materialbillboard)))) "None"))
      (`SceneComponent.SetVisibility` _materialbillboard1 true false)
      (bind _returnvalue_2 (`PrimitiveComponent.CreateDynamicMaterialInstance` _materialbillboard1 0 (`.Material` (break `MaterialSpriteElement` (`|GetArrayItem` (`MaterialBillboardComponent.Elements` _materialbillboard1)))) "None"))
      (`|ExecutionSequence`
        (:`then_0`
          (bind (_direction_5 _newtrack_0_5) (`Timeline|Timeline_3` :!via `PlayFromStart`)
            (:`Update`
              (`MaterialInstanceDynamic.SetScalarParameterValue` _returnvalue "OpStr" _newtrack_0_5))))
        (:`then_1`
          (bind (_direction_6 _newtrack_0_6) (`Timeline|Timeline_5` :!via `PlayFromStart`)
            (:`Update`
              (`MaterialInstanceDynamic.SetScalarParameterValue` _returnvalue_2 "OpStr" _newtrack_0_6))))))
    (:`then_2`
      (`KismetSystemLibrary.Delay` 2.0)
      (`SceneComponent.SetVisibility` (`self.Rocket`) false false)
      (`SceneComponent.SetVisibility` (`self.MaterialBillboard`) false false)
      (`SceneComponent.SetVisibility` (`self.MaterialBillboard1`) false false))))

(fn `UserConstructionScript`)