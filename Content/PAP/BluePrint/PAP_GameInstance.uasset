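; PAP_GameInstance is the game instance that sets up persistent settings data when the game starts.
; On Init it loads the SettingsData save slot into SaveSettingsData, or creates and immediately saves a new object if the slot is missing.
; Disconnected chains that never run would spawn and store manager actors for saves, delegates, gifts, cannonballs and skins, plus a video player and a hierarchical duck actor.
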(event `self.ReceiveInit`
  (`|ExecutionSequence`
    (:`then_3`
      (bind _returnvalue (`GameplayStatics.DoesSaveGameExist` "SettingsData"))
      (if _returnvalue
        (bind _returnvalue_2 (`GameplayStatics.LoadGameFromSlot` "SettingsData"))
        (bind _assettings_data (cast `/Game/PAP/UI/ConfigData/SettingsData` _returnvalue_2))
        (set `self.Save_SettingsData` _assettings_data)
        (else
          (bind _returnvalue_3 (`GameplayStatics.CreateSaveGameObject` "/Game/PAP/UI/ConfigData/SettingsData.SettingsData_C"))
          (bind _output_get (set `self.Save_SettingsData` _returnvalue_3))
          (`GameplayStatics.SaveGameToSlot` _output_get "SettingsData"))))))