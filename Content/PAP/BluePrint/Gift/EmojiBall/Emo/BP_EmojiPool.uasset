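; BP_EmojiPool is an object pool actor for physics-driven BP_Emo emoji balls.
; Tick pre-fills the pool one spawn per frame up to 500, spreading the cost over time.
; BackEmojiToPool stores a ball, disables its physics, gravity and collision, hides it and teleports it to PoolLoc.
; GetEmojiFromPool pops the last entry, re-enables those settings and returns it, with no empty-pool refill.
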(event `self.ReceiveTick`
  (params (DeltaSeconds :type "Float (single-precision)"))
  (if (< (`self.Index`) 500)
    (bind _returnvalue (`|SpawnActorFromClass` "/Game/PAP/BluePrint/Gift/EmojiBall/Emo/BP_Emo.BP_Emo_C" (`KismetMathLibrary.MakeTransform` (`self.PoolLoc`)) "Undefined" "MultiplyWithRoot" null null))
    (`self.BackEmojiToPool` _returnvalue)
    (`/Engine/EditorBlueprintResources/StandardMacros.IncrementInt` (`self.Index`))))

(fn `BackEmojiToPool`
  (params (`Actor Emoji Ref` :type "/Game/PAP/BluePrint/Gift/EmojiBall/Emo/BP_Emo Object Reference"))
  (bind _emojiball (`/Game/PAP/BluePrint/Gift/EmojiBall/Emo/BP_Emo.EmojiBall` `Actor Emoji Ref`))
  (`KismetArrayLibrary.Array_Add` (`self.EmojiPool`) `Actor Emoji Ref`)
  (`/Engine/EditorBlueprintResources/StandardMacros.IsValid` _emojiball
    (:`Is Valid`
      (`PrimitiveComponent.SetSimulatePhysics` _emojiball false)
      (`PrimitiveComponent.SetEnableGravity` _emojiball false)
      (`PrimitiveComponent.SetCollisionEnabled` _emojiball "NoCollision")
      (`SceneComponent.SetVisibility` _emojiball false false)
      (`SceneComponent.K2_SetWorldLocation` _emojiball (`self.PoolLoc`) false true))))

(fn `GetEmojiFromPool`
  (returns (`Last Emoji` :type "/Game/PAP/BluePrint/Gift/EmojiBall/Emo/BP_Emo Object Reference"))
  (bind _last_emoji (`self.Pop`))
  (`/Engine/EditorBlueprintResources/StandardMacros.IsValid` _last_emoji
    (:`Is Valid`
      (bind _emojiball (`/Game/PAP/BluePrint/Gift/EmojiBall/Emo/BP_Emo.EmojiBall` _last_emoji))
      (`PrimitiveComponent.SetCollisionEnabled` _emojiball "QueryAndPhysics")
      (`PrimitiveComponent.SetEnableGravity` _emojiball true)
      (`PrimitiveComponent.SetSimulatePhysics` _emojiball true)
      (`SceneComponent.SetVisibility` _emojiball true false)
      (return _last_emoji))))

(fn `Pop`
  (returns (`Last Emoji` :type "/Game/PAP/BluePrint/Gift/EmojiBall/Emo/BP_Emo Object Reference"))
  (locals (`Last Emoji Ref` :type "/Game/PAP/BluePrint/Gift/EmojiBall/Emo/BP_Emo Object Reference"))
  (bind _emojipool (`self.EmojiPool`))
  (bind _output_get (set `local.Last Emoji Ref` (`|GetArrayItem` _emojipool (`KismetArrayLibrary.Array_LastIndex` _emojipool))))
  (`KismetArrayLibrary.Array_RemoveItem` _emojipool _output_get)
  (return (`local.Last Emoji Ref`)))

(fn `UserConstructionScript`)