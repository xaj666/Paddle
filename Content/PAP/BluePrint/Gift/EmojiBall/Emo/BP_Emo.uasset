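; Emoji ball projectile with a random mesh that homes in on the player's boat (BP_PawnBoat).
; Each tick it steers toward the boat's LocationTaker at constant speed.
; Hitting the player-controlled boat adds a horizontal velocity push and spawns a Niagara effect.
; A hit or one-second timeout disarms it once: homing stops, gravity and damping take over, physics later freezes, and the actor eventually destroys itself.
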(event `self.ReceiveBeginPlay`
  (bind _emojiball (`self.EmojiBall`))
  (bind _emojiball_2 (`self.EmojiBall`))
  (bind _asbp_pawn_boat (cast `/Game/PAP/BluePrint/BP_PawnBoat` (`GameplayStatics.GetPlayerPawn` 0)))
  (set `self.BoatRef` _asbp_pawn_boat)
  (`PrimitiveComponent.SetPhysicsLinearVelocity` (`self.EmojiBall`) (* (`self.GetActorForwardVector`) 2000) false "None")
  (`KismetSystemLibrary.Delay` 1.0)
  ;[1 1 1] 表情子弹失能
  (`/Engine/EditorBlueprintResources/StandardMacros.DoOnce` false :!label _label
    (:`Completed`
      (`|ExecutionSequence`
        (:`then_0`
          (`self.SetActorTickEnabled` false)
          (`PrimitiveComponent.SetEnableGravity` _emojiball_2 true)
          (`PrimitiveComponent.SetCollisionResponseToChannel` _emojiball_2 "ECC_WorldStatic" "ECR_Block")
          (`PrimitiveComponent.SetCollisionResponseToChannel` _emojiball_2 "ECC_WorldDynamic" "ECR_Block")
          (`PrimitiveComponent.SetCollisionResponseToChannel` _emojiball_2 "ECC_PhysicsBody" "ECR_Ignore"))
        (:`then_1`
          (`PrimitiveComponent.SetAngularDamping` _emojiball 1.0)
          (`PrimitiveComponent.SetLinearDamping` _emojiball 1.0)
          (`KismetSystemLibrary.Delay` 2.0)
          (`PrimitiveComponent.SetSimulatePhysics` (`self.EmojiBall`) false)
          (set `self.Not HIt Character Yet?` false))
        (:`then_2`
          (`KismetSystemLibrary.Delay` 30.0)
          (`self.K2_DestroyActor`))))))

(event `self.ReceiveTick`
  (params (DeltaSeconds :type "Float (single-precision)"))
  (bind _emojiball (`self.EmojiBall`))
  (bind _returnvalue (`KismetMathLibrary.RInterpTo` (`SceneComponent.K2_GetComponentRotation` _emojiball) (`KismetMathLibrary.FindLookAtRotation` (`SceneComponent.K2_GetComponentLocation` _emojiball) (`SceneComponent.K2_GetComponentLocation` (`/Game/PAP/BluePrint/BP_PawnBoat.Location Taker` (`self.BoatRef`)))) 0.033333 50.0))
  (`SceneComponent.K2_SetWorldRotation` _emojiball _returnvalue false false)
  (`PrimitiveComponent.SetPhysicsLinearVelocity` (`self.EmojiBall`) (* (`KismetMathLibrary.Conv_RotatorToVector` _returnvalue) 2000) false "None"))

(event `self.EmojiBall.OnComponentHit`
  (params (HitComponent :type "PrimitiveComponent Object Reference") (OtherActor :type "Actor Object Reference") (OtherComp :type "PrimitiveComponent Object Reference") (NormalImpulse :type "Vector Structure") (Hit :type "HitResult Structure (by ref)"))
  (bind _boatref (`self.BoatRef`))
  (bind (_returnvalue_x _returnvalue_y) (`KismetMathLibrary.BreakVector` (`SceneComponent.K2_GetComponentLocation` (`self.EmojiBall`))))
  (bind (_returnvalue_x_2 _returnvalue_y_2) (`KismetMathLibrary.BreakVector` (`self.K2_GetActorLocation` (`self.BoatRef`))))
  (if (`self.In Use?`)
    (if (`self.Not HIt Character Yet?`)
      (bind _asbp_pawn_boat (cast `/Game/PAP/BluePrint/BP_PawnBoat` OtherActor)
        (:`then`
          (if (`Pawn.IsPlayerControlled` _asbp_pawn_boat)
            (`/Engine/EditorBlueprintResources/StandardMacros.DoOnce` false
              (:`Completed`
                (set `/Game/PAP/BluePrint/BP_PawnBoat.Velocity` (+ (`/Game/PAP/BluePrint/BP_PawnBoat.Velocity` _boatref) (* (`KismetMathLibrary.Normal` (- (`KismetMathLibrary.MakeVector` _returnvalue_x_2 _returnvalue_y_2) (`KismetMathLibrary.MakeVector` _returnvalue_x _returnvalue_y))) 50)) _boatref)
                (`NiagaraFunctionLibrary.SpawnSystemAtLocation` "/Game/PAP/BluePrint/Gift/EmojiBall/NS_Hit_10.NS_Hit_10" (`SceneComponent.K2_GetComponentLocation` (`/Game/PAP/BluePrint/BP_PawnBoat.Location Taker` (`self.BoatRef`))) (struct) (0.1 0.1 0.1))
                (goto _label)))
            (else
              (goto _label))))
        (:`CastFailed`
          (goto _label))))))

(fn `UserConstructionScript`
  (bind _outitem (`KismetArrayLibrary.Array_Random` (`self.Meshs`)))
  (if (`KismetSystemLibrary.IsValid` _outitem)
    (`StaticMeshComponent.SetStaticMesh` (`self.StaticMesh`) _outitem)))