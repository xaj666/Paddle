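; BP_Scharnhorst is a gift NPC that chases the player's boat while firing, apparently emoji balls.
; On BeginPlay it caches the save manager, emoji pool and boat, and restarts the gift manager's Scharnhorst time counter.
; Each Tick it turns toward the boat, advances until within range, and spawns an actor at its gun on a short timer, with audio at saved effect volume.
; Pool retrieval is left unconnected, so shots use SpawnActor.
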(event `self.ReceiveBeginPlay`
  (bind _returnvalue (`GameplayStatics.GetActorOfClass` "/Game/PAP/BluePrint/Manager/BP_SaveManager.BP_SaveManager_C"))
  (bind _output_get (set `self.SaveManagerRef` _returnvalue))
  (bind _returntotal___effectmusic (`/Game/PAP/BluePrint/Manager/BP_SaveManager.GetEffectMusic` _output_get))
  (bind _returnvalue_2 (`AddComponent|NODE_AddAudioComponent-0`))
  (`AudioComponent.SetVolumeMultiplier` _returnvalue_2 _returntotal___effectmusic)
  (bind _returnvalue_3 (`GameplayStatics.GetActorOfClass` "/Game/PAP/BluePrint/Gift/EmojiBall/Emo/BP_EmojiPool.BP_EmojiPool_C"))
  (set `self.EmojiPool` _returnvalue_3)
  (bind _returnvalue_4 (`GameplayStatics.GetActorOfClass` "/Game/PAP/BluePrint/Gift/BP_GiftManager.BP_GiftManager_C"))
  (set `/Game/PAP/BluePrint/Gift/BP_GiftManager.ScharmhorstTimer` 0.0 _returnvalue_4)
  (set `/Game/PAP/BluePrint/Gift/BP_GiftManager.ScharnhorstTimeCounterOpen?` true _returnvalue_4)
  (bind _returnvalue_5 (`GameplayStatics.GetActorOfClass` "/Game/PAP/BluePrint/BP_PawnBoat.BP_PawnBoat_C"))
  (set `self.BoatRef` _returnvalue_5))

(event `self.ReceiveTick`
  (params (DeltaSeconds :type "Float (single-precision)"))
  (bind _npc (`self.NPC`))
  (bind (_returnvalue_roll _returnvalue_pitch _returnvalue_yaw) (`KismetMathLibrary.BreakRotator` (`KismetMathLibrary.FindLookAtRotation` (`SceneComponent.K2_GetComponentLocation` (`self.NPC`)) (`SceneComponent.K2_GetComponentLocation` (`/Game/PAP/BluePrint/BP_PawnBoat.Location Taker` (`self.BoatRef`))))))
  (`|ExecutionSequence`
    (:`then_0`
      ;[1 1 1] 面向玩家
      (`SceneComponent.K2_SetWorldRotation` (`self.NPC`) (`KismetMathLibrary.MakeRotator` _returnvalue_roll _returnvalue_pitch (+ _returnvalue_yaw -90.0)) false false)
      (set `self.Distance` (`KismetMathLibrary.VSize` (- (`SceneComponent.K2_GetComponentLocation` (`self.NPC`)) (`SceneComponent.K2_GetComponentLocation` (`/Game/PAP/BluePrint/BP_PawnBoat.Location Taker` (`self.BoatRef`))))))
      (if (> (`self.Distance`) 300.0)
        (`SceneComponent.K2_AddWorldOffset` _npc (* (`SceneComponent.GetRightVector` _npc) 5.0) false false)))
    (:`then_1`
      ;[1 1 1] 间隔生成表情球
      (if (> (`self.SpawnTimer`) 0.0)
        (set `self.SpawnTimer` (- (`self.SpawnTimer`) (`GameplayStatics.GetWorldDeltaSeconds`)))
        (else
          (set `self.SpawnTimer` 0.1)
          (`|SpawnActorFromClass` "/Game/PAP/BluePrint/Gift/EmojiBall/Emo/BP_Emo.BP_Emo_C" (`KismetMathLibrary.MakeTransform` (`SceneComponent.K2_GetComponentLocation` (`self.Gun`))) "Undefined" "MultiplyWithRoot" null null)
          (bind _returnvalue (`AddComponent|NODE_AddAudioComponent-1`))
          (bind _returntotal___effectmusic (`/Game/PAP/BluePrint/Manager/BP_SaveManager.GetEffectMusic` (`self.SaveManagerRef`)))
          (`AudioComponent.SetVolumeMultiplier` _returnvalue _returntotal___effectmusic))))))

(fn `UserConstructionScript`)