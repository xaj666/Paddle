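; Gift water mine that counts down on camera-facing text, then explodes with particles and camera shake.
; If BP_PawnBoat is within range and GiftManager's 金钟罩 (Golden Bell) shield is off, the blast sets its horizontal velocity away from the mine.
; Tick also detects water landings by mesh height for splash effects and runs delayed destruction when a hit sets Destory.
; A timeline triggers flashes, and ImpactEffectSpawn provides a boat-oriented hit effect.
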(event `self.ReceiveBeginPlay`
  (bind _returnvalue (`GameplayStatics.GetActorOfClass` "/Game/PAP/BluePrint/BP_PawnBoat.BP_PawnBoat_C"))
  (set `self.BoatRef` _returnvalue)
  (bind _returnvalue_2 (`GameplayStatics.GetActorOfClass` "/Game/PAP/BluePrint/Gift/BP_GiftManager.BP_GiftManager_C"))
  (set `self.GiftManagerRef` _returnvalue_2)
  (`KismetSystemLibrary.Delay` 0.2)
  (bind _returnvalue_3 (`AddComponent|NODE_AddAudioComponent-0`))
  (set `self.AudioRef` _returnvalue_3)
  (`AudioComponent.Play` _returnvalue_3 0.0)
  (`Timeline|时间轴`
    (:`事件轨道`
      (`NiagaraFunctionLibrary.SpawnSystemAtLocation` "/Game/PAP/Special_Effect/redflashc4/FX/flashc4.flashc4" (`SceneComponent.K2_GetComponentLocation` (`self.WaterMine Mesh`)) (struct) (0.3 0.3 0.3) true true "AutoRelease"))))

(event `self.ReceiveTick`
  (params (DeltaSeconds :type "Float (single-precision)"))
  (bind _watermine_mesh (`self.WaterMine Mesh`))
  (bind _watermine_mesh_2 (`self.WaterMine Mesh`))
  (bind (_returnvalue_x _returnvalue_y _returnvalue_z) (`KismetMathLibrary.BreakVector` (`SceneComponent.K2_GetComponentLocation` _watermine_mesh_2)))
  (bind (_returnvalue_x_2 _returnvalue_y_2 _returnvalue_z_2) (`KismetMathLibrary.BreakVector` (`SceneComponent.K2_GetComponentLocation` _watermine_mesh)))
  (bind (_returnvalue_roll _returnvalue_pitch _returnvalue_yaw) (`KismetMathLibrary.BreakRotator` (`KismetMathLibrary.FindLookAtRotation` (`SceneComponent.K2_GetComponentLocation` (`self.TimeCounter`)) (`SceneComponent.K2_GetComponentLocation` (`/Game/PAP/BluePrint/BP_PawnBoat.Camera` (`self.BoatRef`))))))
  (set `self.Delta Seconds` DeltaSeconds)
  (if (> (`self.MaxCountTime`) 0.0)
    (bind _output_get (set `self.MaxCountTime` (- (`self.MaxCountTime`) DeltaSeconds)))
    (`TextRenderComponent.K2_SetText` (`self.TimeCounter`) (`KismetTextLibrary.Conv_Int64ToText` (`KismetMathLibrary.FFloor64` _output_get)))
    (`SceneComponent.K2_SetWorldRotation` (`self.TimeCounter`) (`KismetMathLibrary.MakeRotator` _returnvalue_roll 0.0 _returnvalue_yaw) false false)
    (`|ExecutionSequence`
      (:`then_0`
        ;[1 1 1] 由击打动作触发
        (if (`self.Destory?`)
          (if (> (`self.DestroyTimeCount`) 0.0)
            (set `self.DestroyTimeCount` (- (`self.DestroyTimeCount`) (`self.Delta Seconds`)))
            (else
              (`ActorComponent.K2_DestroyComponent` (`self.AudioRef`))
              (`self.K2_DestroyActor`)))))
      (:`then_1`
        (`|ExecutionSequence`
          (:`then_0`
            ;[1 1 1] 落水检测
            (`/Engine/EditorBlueprintResources/StandardMacros.IsValid` _watermine_mesh
              (:`Is Valid`
                (bind _output_get_2 (set `self.WaterMineHeight` _returnvalue_z_2))
                (if (> _output_get_2 0.0)
                  (set `self.IsIntheAir?` true)))))
          (:`then_1`
            ;[1 1 1] 落水特效释放
            (if (`self.IsIntheAir?`)
              (if (< (`self.WaterMineHeight`) -20.0)
                (`NiagaraFunctionLibrary.SpawnSystemAtLocation` "/Game/PAP/Special_Effect/SplashesFxPack/Effects/Wave_SE.Wave_SE" (`SceneComponent.K2_GetComponentLocation` (`self.WaterMine Mesh`)))
                (`AddComponent|NODE_AddAudioComponent-2`)
                (set `self.IsIntheAir?` false)))))))
    (else
      ;[1 1 1] 单次触发
      (if (`self.Pass?`)
        (`|ExecutionSequence`
          (:`then_0`
            (`SceneComponent.ToggleVisibility` _watermine_mesh_2 false)
            (`SceneComponent.ToggleVisibility` (`self.TimeCounter`) false)
            (bind (_inrange_ _distance_to_player) (`self.Calculate Distance`))
            (if _inrange_
              (bind `_金钟罩开启_` (`/Game/PAP/BluePrint/Gift/BP_GiftManager.金钟罩开启?` (`self.GiftManagerRef`)))
              (if (not `_金钟罩开启_`)
                (`self.Apply Impluse` _distance_to_player)))
            (`KismetSystemLibrary.Delay` 3.0)
            (`self.K2_DestroyActor`))
          (:`then_1`
            (`GameplayStatics.SpawnEmitterAtLocation` "/Game/PAP/Special_Effect/CartoonyFXPACK4/Particles/FX/PS_Boom2.PS_Boom2" (`KismetMathLibrary.MakeVector` _returnvalue_x _returnvalue_y (+ _returnvalue_z 0.0))))
          (:`then_2`
            (`PlayerCameraManager.StartCameraShake` :`self` (`GameplayStatics.GetPlayerCameraManager` 0) :`ShakeClass` "/Game/PAP/BluePrint/CameraShake/BP_CameraShakeForWaterMine.BP_CameraShakeForWaterMine_C")
            (set `self.Pass?` false)))))))

(fn `Apply Impluse`
  (params (Distance :type "Vector Structure"))
  (bind (_returnvalue_x _returnvalue_y) (`KismetMathLibrary.BreakVector` (`KismetMathLibrary.Normal` Distance)))
  (bind _returnvalue (`GameplayStatics.GetActorOfClass` "/Game/PAP/BluePrint/BP_PawnBoat.BP_PawnBoat_C"))
  (set `/Game/PAP/BluePrint/BP_PawnBoat.Velocity` (* (`KismetMathLibrary.MakeVector` _returnvalue_x _returnvalue_y) (`self.ExplosionForce`)) _returnvalue))

(fn `Calculate Distance`
  (returns (`InRange?` :type Boolean) (`Distance To Player` :type "Vector Structure"))
  (locals (`Distance From Mine to Player` :type "Vector Structure"))
  (bind _returnvalue (- (`SceneComponent.K2_GetComponentLocation` (`/Game/PAP/BluePrint/BP_PawnBoat.BoatMesh` (`self.BoatRef`))) (`SceneComponent.K2_GetComponentLocation` (`self.WaterMine Mesh`))))
  (bind _output_get (set `local.Distance From Mine to Player` _returnvalue))
  (return (< (`KismetMathLibrary.VSize` _returnvalue) (`self.ExplosionRange`)) _output_get))

(fn `ImpactEffectSpawn`
  (`GameplayStatics.SpawnEmitterAtLocation` "/Game/PAP/Special_Effect/MyEffect/Impact_SE_WaterMine.Impact_SE_WaterMine" (`SceneComponent.K2_GetComponentLocation` (`self.WaterMine Mesh`)) (`KismetMathLibrary.ComposeRotators` (`KismetMathLibrary.FindLookAtRotation` (`SceneComponent.K2_GetComponentLocation` (`self.WaterMine Mesh`)) (`SceneComponent.K2_GetComponentLocation` (`/Game/PAP/BluePrint/BP_PawnBoat.Location Taker` (`self.BoatRef`)))) (struct :`Pitch` -90.0)) (0.3 0.3 0.3)))

(fn `UserConstructionScript`)