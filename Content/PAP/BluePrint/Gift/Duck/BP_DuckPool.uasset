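; Object pool actor that pre-spawns and recycles BP_ActorDuck instances to be handed out on request.
; Tick spawns one duck per frame until the index reaches 600, spreading the cost, and sends each straight into the pool.
; GetDuckFromPool pops the last entry and enables its collision, physics, gravity and visibility.
; BackDuckToPool stores a duck, disables those same properties and teleports it to the pool location.
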(event `self.ReceiveBeginPlay`)

(event `self.ReceiveTick`
  (params (DeltaSeconds :type "Float (single-precision)"))
  (if (< (`self.index`) 600)
    (bind _returnvalue (`|SpawnActorFromClass` "/Game/PAP/BluePrint/Gift/Duck/BP_ActorDuck.BP_ActorDuck_C" (`KismetMathLibrary.MakeTransform` (`self.PoolLoc`)) "Undefined" "MultiplyWithRoot" null null))
    (`self.BackDuckToPool` _returnvalue)
    (`/Engine/EditorBlueprintResources/StandardMacros.IncrementInt` (`self.index`))))

(fn `BackDuckToPool`
  (params (`Actor Duck Ref` :type "/Game/PAP/BluePrint/Gift/Duck/BP_ActorDuck Object Reference (by ref)"))
  (bind _duck (`/Game/PAP/BluePrint/Gift/Duck/BP_ActorDuck.Duck` `Actor Duck Ref`))
  (`KismetArrayLibrary.Array_Add` (`self.DuckPool`) `Actor Duck Ref`)
  (`/Engine/EditorBlueprintResources/StandardMacros.IsValid` _duck
    (:`Is Valid`
      (`PrimitiveComponent.SetSimulatePhysics` _duck false)
      (`PrimitiveComponent.SetEnableGravity` _duck false)
      (`PrimitiveComponent.SetCollisionEnabled` _duck "NoCollision")
      (`SceneComponent.SetVisibility` _duck false false)
      (`SceneComponent.K2_SetWorldLocation` _duck (`self.PoolLoc`) false true))))

(fn `GetDuckFromPool`
  (returns (`Duck Actor Ref` :type "/Game/PAP/BluePrint/Gift/Duck/BP_ActorDuck Object Reference"))
  (bind _duck_actor_ref (`self.Pop` (`self.DuckPool`)))
  (`/Engine/EditorBlueprintResources/StandardMacros.IsValid` _duck_actor_ref
    (:`Is Valid`
      (bind _duck (`/Game/PAP/BluePrint/Gift/Duck/BP_ActorDuck.Duck` _duck_actor_ref))
      (`PrimitiveComponent.SetCollisionEnabled` _duck "QueryAndPhysics")
      (`PrimitiveComponent.SetEnableGravity` _duck true)
      (`PrimitiveComponent.SetSimulatePhysics` _duck true)
      (`SceneComponent.SetVisibility` _duck true false)
      (return _duck_actor_ref))))

(fn `Pop`
  (params (DuckPool :type "Array of /Game/PAP/BluePrint/Gift/Duck/BP_ActorDuck Object Reference"))
  (returns (`Duck Actor Ref` :type "/Game/PAP/BluePrint/Gift/Duck/BP_ActorDuck Object Reference"))
  (locals (LastRef :type "/Game/PAP/BluePrint/Gift/Duck/BP_ActorDuck Object Reference"))
  (bind _output_get (set `local.LastRef` (`|GetArrayItem` DuckPool (`KismetArrayLibrary.Array_LastIndex` DuckPool))))
  (`KismetArrayLibrary.Array_RemoveItem` DuckPool _output_get)
  (return (`local.LastRef`)))

(fn `UserConstructionScript`)