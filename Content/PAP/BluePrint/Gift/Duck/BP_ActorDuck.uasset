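; BP_ActorDuck is a pooled duck actor, tied to the gift system, that detects water landings.
; While in use, it watches its height and on dropping into water spawns a wave effect with volume-scaled audio.
; When its countdown expires, it returns to the manager's pool, first leaving a hierarchical instanced mesh copy unless AirBorne.
; ImapactEffect spawns a water-mine emitter rotated relative to the boat.
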(event `self.ReceiveBeginPlay`
  (bind _returnvalue (`GameplayStatics.GetActorOfClass` "/Game/PAP/BluePrint/Gift/Duck/BP_Hirerarchilcal_Duck.BP_Hirerarchilcal_Duck_C"))
  (set `self.Hier Ref` _returnvalue)
  (set `self.Hierarchical Instanced Static Mesh` (`/Game/PAP/BluePrint/Gift/Duck/BP_Hirerarchilcal_Duck.HierarchicalInstancedStaticMesh` _returnvalue))
  (bind _returnvalue_2 (`GameplayStatics.GetActorOfClass` "/Game/PAP/BluePrint/Gift/BP_GiftManager.BP_GiftManager_C"))
  (bind _output_get (set `self.GiftManagerRef` _returnvalue_2))
  (set `self.Duck Pool Ref` (`/Game/PAP/BluePrint/Gift/BP_GiftManager.DuckPoolRef` _output_get))
  (bind _returnvalue_3 (`GameplayStatics.GetActorOfClass` "/Game/PAP/BluePrint/BP_PawnBoat.BP_PawnBoat_C"))
  (set `self.BoatRef` _returnvalue_3)
  (bind _returnvalue_4 (`GameplayStatics.GetActorOfClass` "/Game/PAP/BluePrint/Manager/BP_SaveManager.BP_SaveManager_C"))
  (set `self.SaveManagerRef` _returnvalue_4))

(event `self.ReceiveTick`
  (params (DeltaSeconds :type "Float (single-precision)"))
  (if (`self.IsBeingUsed?`)
    (set `self.Delta Seconds` DeltaSeconds)
    (`|ExecutionSequence`
      (:`then_0`
        (`self.LandedDectected`))
      (:`then_1`
        (if (> (`self.TimeCount`) 0.0)
          (set `self.TimeCount` (- (`self.TimeCount`) (`self.Delta Seconds`)))
          (else
            (set `self.TimeCount` 5.0)
            (if (not (`self.AirBorne?`))
              (`/Game/PAP/BluePrint/Gift/Duck/BP_Hirerarchilcal_Duck.Add /Show Instance` (`self.Hier Ref`) (`SceneComponent.K2_GetComponentToWorld` (`self.Duck`))))
            (`/Game/PAP/BluePrint/Gift/Duck/BP_DuckPool.BackDuckToPool` (`self.Duck Pool Ref`) self)
            (set `self.IsBeingUsed?` false)
            (set `self.AirBorne?` false)))))))

(fn `ImapactEffect`
  (`GameplayStatics.SpawnEmitterAtLocation` "/Game/PAP/Special_Effect/MyEffect/Impact_SE_WaterMine.Impact_SE_WaterMine" (`SceneComponent.K2_GetComponentLocation` (`self.Duck`)) (`KismetMathLibrary.ComposeRotators` (`KismetMathLibrary.FindLookAtRotation` (`SceneComponent.K2_GetComponentLocation` (`self.Duck`)) (`SceneComponent.K2_GetComponentLocation` (`/Game/PAP/BluePrint/BP_PawnBoat.Location Taker` (`self.BoatRef`)))) (struct :`Pitch` -90.0)) (0.3 0.3 0.3)))

(fn `LandedDectected`
  (locals (DuckHeight :type "Float (double-precision)" :default 0.0))
  (bind (_returnvalue_x _returnvalue_y _returnvalue_z) (`KismetMathLibrary.BreakVector` (`SceneComponent.K2_GetComponentLocation` (`self.Duck`))))
  (`|ExecutionSequence`
    (:`then_0`
      ;[1 1 1] 落水检测
      (bind _output_get (set `local.DuckHeight` _returnvalue_z))
      (if (> _output_get 0.0)
        (set `self.IsIntheAir?` true)))
    (:`then_1`
      ;[1 1 1] 落水特效释放
      (if (`self.IsIntheAir?`)
        (if (< (`local.DuckHeight`) -10.0)
          (`NiagaraFunctionLibrary.SpawnSystemAtLocation` "/Game/PAP/Special_Effect/SplashesFxPack/Effects/Wave_SE.Wave_SE" (`SceneComponent.K2_GetComponentLocation` (`self.Duck`)))
          (bind _returnvalue (`AddComponent|NODE_AddAudioComponent-1`))
          (bind _returntotal___effectmusic (`/Game/PAP/BluePrint/Manager/BP_SaveManager.GetEffectMusic` (`self.SaveManagerRef`)))
          (`AudioComponent.SetVolumeMultiplier` _returnvalue _returntotal___effectmusic)
          (set `self.IsIntheAir?` false))))))

(fn `UserConstructionScript`)