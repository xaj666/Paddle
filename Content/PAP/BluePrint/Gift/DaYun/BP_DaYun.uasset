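; BP_DaYun is a gift actor that homes in on BP_PawnBoat at fixed speed and rams it.
; On reaching close range it fires once: unless the boat's 金钟罩 shield is on, it sets knockback velocity, spawns an emitter and adds sway for hits along the boat's local X axis.
; It plays impact audio either way, then self-destructs after a delay.
; Each tick its Image also yaws toward the boat camera and pulses in scale.
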(event `self.ReceiveBeginPlay`
  (bind (_returnvalue_x _returnvalue_y) (`KismetMathLibrary.BreakVector` (`SceneComponent.K2_GetComponentLocation` (`self.Location Taker`))))
  (bind _returnvalue (`KismetMathLibrary.MakeVector` _returnvalue_x _returnvalue_y -20.0))
  (bind _returnvalue_2 (`GameplayStatics.GetActorOfClass` "/Game/PAP/BluePrint/BP_PawnBoat.BP_PawnBoat_C"))
  (set `self.BoatRef` _returnvalue_2)
  (set `self.Location Taker` (`/Game/PAP/BluePrint/BP_PawnBoat.Location Taker` _returnvalue_2))
  (set `self.TargetLoc` _returnvalue)
  (set `self.Distance To Target` (`KismetMathLibrary.VSize` (- _returnvalue (`SceneComponent.K2_GetComponentLocation` (`self.DaYun_SM`))))))

(event `self.ReceiveTick`
  (params (DeltaSeconds :type "Float (single-precision)"))
  (bind _boatref (`self.BoatRef`))
  (bind _boatref_2 (`self.BoatRef`))
  (bind _boatref_3 (`self.BoatRef`))
  (bind _image (`self.Image`))
  (bind _returnvalue (`SceneComponent.K2_GetComponentLocation` (`self.DaYun_SM`)))
  (bind _returnvalue_2 (`SceneComponent.K2_GetComponentLocation` (`self.DaYun_SM`)))
  (bind (_returnvalue_x _returnvalue_y) (`KismetMathLibrary.BreakVector` (`SceneComponent.K2_GetComponentLocation` (`self.Location Taker`))))
  (bind _returnvalue_3 (* (`self.ScaleValue`) (`self.ScaleStepLength`)))
  (bind _swayvelocity (`/Game/PAP/BluePrint/BP_PawnBoat.SwayVelocity` _boatref_2))
  (bind _swayimpuse (`/Game/PAP/BluePrint/BP_PawnBoat.SwayImpuse` _boatref_2))
  (bind _returnvalue_4 (`SceneComponent.K2_GetComponentLocation` (`/Game/PAP/BluePrint/BP_PawnBoat.Location Taker` _boatref)))
  (bind (_returnvalue_roll _returnvalue_pitch _returnvalue_yaw) (`KismetMathLibrary.BreakRotator` (`KismetMathLibrary.FindLookAtRotation` (`SceneComponent.K2_GetComponentLocation` _image) (`SceneComponent.K2_GetComponentLocation` (`/Game/PAP/BluePrint/BP_PawnBoat.Camera` (`self.BoatRef`))))))
  (bind _returnvalue_5 (- (`KismetMathLibrary.MakeVector` _returnvalue_x _returnvalue_y -20.0) _returnvalue))
  (bind (_returnvalue_x_2 _returnvalue_y_2) (`KismetMathLibrary.BreakVector` (- _returnvalue_4 _returnvalue_2)))
  (bind (_returnvalue_x_3 _returnvalue_y_3) (`KismetMathLibrary.BreakVector` (`KismetMathLibrary.LessLess_VectorRotator` (`KismetMathLibrary.Normal` (- (`SceneComponent.K2_GetComponentLocation` (`self.DaYun_SM`)) (`SceneComponent.K2_GetComponentLocation` (`/Game/PAP/BluePrint/BP_PawnBoat.Location Taker` _boatref_3)))) (`self.K2_GetActorRotation` _boatref_3))))
  (`|ExecutionSequence`
    (:`then_0`
      ;[1 1 1] 乌萨奇生成后
      (if (`self.IsCloseEnoughToTarget?`)
        (if (`self.Condition`)
          ;;[1 1 1] 仅执行一次
          (if (not (`/Game/PAP/BluePrint/BP_PawnBoat.金钟罩开启?` _boatref))
            (set `/Game/PAP/BluePrint/BP_PawnBoat.Velocity` (* (`self.CrushForce`) (`KismetMathLibrary.MakeVector` _returnvalue_x_2 _returnvalue_y_2)) (`self.BoatRef`))
            (`GameplayStatics.SpawnEmitterAtLocation` "/Game/PAP/Special_Effect/SmokeFX/Particles/P_MuzzleFlashA_01.P_MuzzleFlashA_01" _returnvalue_2 (`KismetMathLibrary.ComposeRotators` (`KismetMathLibrary.FindLookAtRotation` _returnvalue_4 _returnvalue_2) (struct :`Pitch` -90.0)))
            ;;;[0.1215 0.1406 0.1303] 计算被撞后船的侧倾方向
            (set `self.ABS_X` 0.0)
            (set `self.ABS_Y` 0.0)
            (if (> (`KismetMathLibrary.Abs` _returnvalue_y_3) (`KismetMathLibrary.Abs` _returnvalue_x_3))
              _
              (elif (< _returnvalue_x_3 0.0)
                ;;;[0.08854 0.08854 0.08854] 应用侧倾
                (set `/Game/PAP/BluePrint/BP_PawnBoat.SwayVelocity` (- _swayvelocity _swayimpuse) _boatref_2)
                (else
                  (set `/Game/PAP/BluePrint/BP_PawnBoat.SwayVelocity` (+ _swayvelocity _swayimpuse) _boatref_2)))))
          (set `self.Condition` false)
          (bind _returnvalue_6 (`AddComponent|NODE_AddAudioComponent-0`))
          (`AudioComponent.SetVolumeMultiplier` _returnvalue_6 (`/Game/PAP/BluePrint/BP_PawnBoat.FinalEffectSoundVolume` (`self.BoatRef`)))
          (else
            ;[1 1 1] 上述逻辑结束后，销毁
            (`KismetSystemLibrary.Delay` 1.0)
            (`self.K2_DestroyActor`)))
        (else
          ;;[1 1 1] 值更新
          (set `self.CurrentLoc` _returnvalue)
          (set `self.Distance To Target` (`KismetMathLibrary.VSize` _returnvalue_5))
          (`SceneComponent.K2_SetWorldLocation` (`self.DaYun_SM`) (+ (* (* (`KismetMathLibrary.Normal` _returnvalue_5) DeltaSeconds) (`self.Speed`)) (`self.CurrentLoc`)) false false)
          (if (< (`self.Distance To Target`) 70.0)
            (set `self.IsCloseEnoughToTarget?` true)))))
    (:`then_1`
      ;[1 1 1] 文字朝向
      (`SceneComponent.K2_SetWorldRotation` _image (`KismetMathLibrary.MakeRotator` 90.0 0.0 (+ _returnvalue_yaw -90.0)) false false)
      ;[1 1 1] 文字缩放
      (if (`self.IsScalingUp?`)
        (`SceneComponent.SetWorldScale3D` (`self.Image`) (+ (`SceneComponent.K2_GetComponentScale` (`self.Image`)) _returnvalue_3))
        (set `self.ScaleDepth` (+ (`self.ScaleDepth`) 1.5))
        (if (> (`self.ScaleDepth`) 10.0)
          (set `self.IsScalingUp?` false))
        (else
          (`SceneComponent.SetWorldScale3D` (`self.Image`) (- (`SceneComponent.K2_GetComponentScale` (`self.Image`)) _returnvalue_3))
          (set `self.ScaleDepth` (- (`self.ScaleDepth`) 1.5))
          (if (< (`self.ScaleDepth`) 0.0)
            (set `self.IsScalingUp?` true)))))))

(fn `UserConstructionScript`)