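; BP_FuZhou is a gift talisman (符咒) projectile that homes in on and sticks to one of the boat pawn's two skeletons.
; BeginPlay picks a random side and upper-body bone; Tick steps toward that bone while Condition holds, box-tracing for the matching L/R-tagged component.
; On a hit it attaches to the bone, stops ticking, triggers a randomly flagged BP_GiftManager effect and camera shake, then destroys itself after a long delay.
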(event `self.ReceiveBeginPlay`
  (bind _boatref (`self.BoatRef`))
  (bind _returnvalue (`GameplayStatics.GetActorOfClass` "/Game/PAP/BluePrint/BP_PawnBoat.BP_PawnBoat_C"))
  (set `self.BoatRef` _returnvalue)
  (bind _returnvalue_2 (`GameplayStatics.GetActorOfClass` "/Game/PAP/BluePrint/Gift/BP_GiftManager.BP_GiftManager_C"))
  (set `self.GiftManagerRef` _returnvalue_2)
  (`|ExecutionSequence`
    (:`then_0`
      (bind _output_get (set `self.BoneIndex` (`KismetMathLibrary.RandomIntegerInRange` 0 7)))
      (switch `int` _output_get
        (:`0`
          (set `self.BoneName` "head"))
        (:`1`
          (set `self.BoneName` "spine_03"))
        (:`2`
          (set `self.BoneName` "upperarm_l"))
        (:`3`
          (set `self.BoneName` "upperarm_r"))
        (:`4`
          (set `self.BoneName` "lowerarm_l"))
        (:`5`
          (set `self.BoneName` "lowerarm_r"))
        (:`6`
          (set `self.BoneName` "clavicle_r"))
        (:`7`
          (set `self.BoneName` "clavicle_l"))))
    (:`then_1`
      (bind _output_get_2 (set `self.Left?` (`KismetMathLibrary.RandomBool`)))
      (if _output_get_2
        (set `self.Target Skeleton` (`/Game/PAP/BluePrint/BP_PawnBoat.Skeleton_L_Display` _boatref))
        (else
          (set `self.Target Skeleton` (`/Game/PAP/BluePrint/BP_PawnBoat.Skeleton_R_Display` _boatref)))))))

(event `self.ReceiveTick`
  (params (DeltaSeconds :type "Float (single-precision)"))
  (bind _returnvalue_location (`KismetMathLibrary.BreakTransform` (`SkinnedMeshComponent.GetBoneTransform` (`self.Target Skeleton`) (`self.BoneName`) "RTS_World")))
  (bind _returnvalue (`SceneComponent.K2_GetComponentLocation` (`self.DefaultSceneRoot`)))
  (if (`self.Condition`)
    (bind _output_get (set `self.TargetBoneLoc` _returnvalue_location))
    (bind _output_get_2 (set `self.Distance` (- _output_get (`SceneComponent.K2_GetComponentLocation` (`self.FuZhou`)))))
    (`SceneComponent.K2_AddWorldOffset` (`self.DefaultSceneRoot`) (* (`KismetMathLibrary.Normal` _output_get_2) 10.0) false false)
    (bind (_outhit _returnvalue_2) (`KismetSystemLibrary.BoxTraceSingleForObjects` _returnvalue _returnvalue (5.0 5.0 5.0) (`self.K2_GetActorRotation` self) (`self.Object Types`) true (`|MakeArray` self :!type "Actor Object Reference") "None" true (struct :`R` 1.0 :`A` 1.0) (struct :`G` 1.0 :`A` 1.0) 1.0))
    (if _returnvalue_2
      (bind (_bblockinghit _binitialoverlap _time _distance _location _impactpoint _normal _impactnormal _physmat _hitactor _hitcomponent) (`GameplayStatics.BreakHitResult` _outhit))
      (cast `/Game/PAP/BluePrint/BP_PawnBoat` _hitactor)
      (if (`self.Left?`)
        (if (`ActorComponent.ComponentHasTag` _hitcomponent "L")
          (`SceneComponent.K2_AttachToComponent` (`self.DefaultSceneRoot`) (`/Game/PAP/BluePrint/BP_PawnBoat.Skeleton_L_Display` (`self.BoatRef`)) (`self.BoneName`) "KeepWorld" "KeepWorld" "KeepWorld" true)
          (set `self.Condition` false :!label _label)
          (`self.SetActorTickEnabled` false)
          (`PrimitiveComponent.SetCollisionEnabled` (`self.FuZhou`) "NoCollision")
          (bind _output_get_3 (set `self.Lei Or Ding` (`KismetMathLibrary.RandomBool`)))
          (if _output_get_3
            (`/Game/PAP/BluePrint/Gift/BP_GiftManager.符咒特效` (`self.GiftManagerRef`) (`SceneComponent.K2_GetComponentLocation` (`self.DefaultSceneRoot`)) self (`self.Lei Or Ding`))
            (else
              (`/Game/PAP/BluePrint/Gift/BP_GiftManager.符咒特效` (`self.GiftManagerRef`) (`SceneComponent.K2_GetComponentLocation` (`self.DefaultSceneRoot`)) self (`self.Lei Or Ding`))
              (`KismetSystemLibrary.Delay` 0.5)))
          (`PlayerCameraManager.StartCameraShake` :`self` (`GameplayStatics.GetPlayerCameraManager` 0) :`ShakeClass` "/Game/PAP/BluePrint/CameraShake/BP_CS_FuZhou.BP_CS_FuZhou_C")
          (`KismetSystemLibrary.Delay` 600.0)
          (`self.K2_DestroyActor`))
        (elif (`ActorComponent.ComponentHasTag` _hitcomponent "R")
          (`SceneComponent.K2_AttachToComponent` (`self.DefaultSceneRoot`) (`/Game/PAP/BluePrint/BP_PawnBoat.Skeleton_R_Display` (`self.BoatRef`)) (`self.BoneName`) "KeepWorld" "KeepWorld" "KeepWorld" true)
          (goto _label))))))

(fn `UserConstructionScript`)