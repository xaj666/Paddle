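; Timeline-driven actor for the FuZhou (符咒, talisman) gift effect, which repeatedly calls the gift manager while moving the player boat vertically.
; On BeginPlay it disables gravity on the boat's LocationTaker and starts a timeline whose event track counts each trigger.
; Tick lifts the boat while Floating is set; later triggers step it downward, then restore gravity with a strong downward velocity.
; The actor destroys itself shortly after the timeline finishes.
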(event `self.ReceiveBeginPlay`
  (bind _boatref (`self.BoatRef`))
  (bind _returnvalue (`GameplayStatics.GetActorOfClass` "/Game/PAP/BluePrint/Gift/BP_GiftManager.BP_GiftManager_C"))
  (set `self.GiftManagerRef` _returnvalue)
  (bind _returnvalue_2 (`GameplayStatics.GetActorOfClass` "/Game/PAP/BluePrint/BP_PawnBoat.BP_PawnBoat_C"))
  (set `self.BoatRef` _returnvalue_2)
  (`PrimitiveComponent.SetEnableGravity` (`/Game/PAP/BluePrint/BP_PawnBoat.Location Taker` (`self.BoatRef`)) false)
  (`Timeline|FuZhouTrigger`
    (:`Finished`
      (`KismetSystemLibrary.Delay` 1.0)
      (`self.K2_DestroyActor`))
    (:`NewTrack_0`
      (`/Game/PAP/BluePrint/Gift/BP_GiftManager.符咒` (`self.GiftManagerRef`))
      (bind _result (`/Engine/EditorBlueprintResources/StandardMacros.IncrementInt` (`self.TriggedTime`))
        (:`  `
          (if (> _result 16)
            (bind _output_get (set `self.floating?` false))
            (if (not (> (`self.TriggedTime`) 31))
              (if (not _output_get)
                (`SceneComponent.K2_AddWorldOffset` (`/Game/PAP/BluePrint/BP_PawnBoat.Location Taker` (`self.BoatRef`)) (0.0 0.0 -40.0) false false))
              (else
                (`PrimitiveComponent.SetEnableGravity` (`/Game/PAP/BluePrint/BP_PawnBoat.Location Taker` _boatref) true)
                (set `/Game/PAP/BluePrint/BP_PawnBoat.Velocity` (0.0 0.0 -3000.0) _boatref)))))))))

(event `self.ReceiveTick`
  (params (DeltaSeconds :type "Float (single-precision)"))
  (if (`self.floating?`)
    (`PrimitiveComponent.SetEnableGravity` (`/Game/PAP/BluePrint/BP_PawnBoat.Location Taker` (`self.BoatRef`)) false)
    (`SceneComponent.K2_AddWorldOffset` (`/Game/PAP/BluePrint/BP_PawnBoat.Location Taker` (`self.BoatRef`)) (0.0 0.0 5.0) false false)))

(fn `UserConstructionScript`)