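; BP_Lei is a short-lived effect actor in the Gift talisman (符咒) folder, built around a Plane component.
; Its root rises a fixed offset every tick, independent of delta time, and the actor destroys itself five seconds after BeginPlay.
; BeginPlay caches the BP_PawnBoat reference, but the logic that would pitch the plane toward that boat's camera is unconnected and never runs.
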(event `self.ReceiveBeginPlay`
  (bind _returnvalue (`GameplayStatics.GetActorOfClass` "/Game/PAP/BluePrint/BP_PawnBoat.BP_PawnBoat_C"))
  (set `self.BoatRef` _returnvalue)
  (`KismetSystemLibrary.Delay` 5.0)
  (`self.K2_DestroyActor`))

(event `self.ReceiveTick`
  (params (DeltaSeconds :type "Float (single-precision)"))
  (`SceneComponent.K2_AddWorldOffset` (`self.DefaultSceneRoot`) (0.0 0.0 1.0) false false))

(fn `UserConstructionScript`)