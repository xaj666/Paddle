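; TianCanJiao gift actor: a foot that takes the camera view on spawn and stomps three times at the player boat before destroying itself.
; Tick oscillates the mesh along its right vector, then decrements the GiftManager's shared instance count.
; The last instance launches the boat horizontally away unless the 金钟罩 shield is active.
; Boat sway depends on local hit direction, and earlier instances apply only sway, ignoring the shield.
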(event `self.ReceiveBeginPlay`
  (set `self.StartLoc` (`SceneComponent.K2_GetComponentLocation` (`self.TianCanJiao`)))
  (bind _returnvalue (`GameplayStatics.GetActorOfClass` "/Game/PAP/BluePrint/BP_PawnBoat.BP_PawnBoat_C"))
  (set `self.BoatRef` _returnvalue)
  (set `self.EndLoc` (`SceneComponent.K2_GetComponentLocation` (`/Game/PAP/BluePrint/BP_PawnBoat.Location Taker` _returnvalue)))
  (bind _returnvalue_2 (`GameplayStatics.GetActorOfClass` "/Game/PAP/BluePrint/Gift/BP_GiftManager.BP_GiftManager_C"))
  (set `self.GiftManagerRef` _returnvalue_2)
  (`/Engine/EditorBlueprintResources/StandardMacros.IncrementInt` (`/Game/PAP/BluePrint/Gift/BP_GiftManager.TianCanJiaoCount` _returnvalue_2)
    (:`  `
      (`PlayerController.SetViewTargetWithBlend` (`PlayerState.GetPlayerController` (`GameplayStatics.GetPlayerState` 0)) self 0.0 "VTBlend_Linear" 0.0 false))))

(event `self.ReceiveTick`
  (params (DeltaSeconds :type "Float (single-precision)"))
  (bind _boatref (`self.BoatRef`))
  (bind _boatref_2 (`self.BoatRef`))
  (bind _tiancanjiaocount (`/Game/PAP/BluePrint/Gift/BP_GiftManager.TianCanJiaoCount` (`self.GiftManagerRef`)))
  (bind _swayvelocity (`/Game/PAP/BluePrint/BP_PawnBoat.SwayVelocity` _boatref))
  (bind _swayimpuse (`/Game/PAP/BluePrint/BP_PawnBoat.SwayImpuse` _boatref))
  (bind _returnvalue (* (`self.FootSpeed`) (`SceneComponent.GetRightVector` (`self.TianCanJiao`))))
  (bind (_returnvalue_x _returnvalue_y) (`KismetMathLibrary.BreakVector` (- (`SceneComponent.K2_GetComponentLocation` (`/Game/PAP/BluePrint/BP_PawnBoat.Location Taker` (`self.BoatRef`))) (`SceneComponent.K2_GetComponentLocation` (`self.TianCanJiao`)))))
  (bind _returnvalue_2 (* -1.0 _returnvalue))
  (bind _returnvalue_3 (* 1.0 _returnvalue))
  (bind (_returnvalue_x_2 _returnvalue_y_2) (`KismetMathLibrary.BreakVector` (`KismetMathLibrary.LessLess_VectorRotator` (`KismetMathLibrary.Normal` (- (`SceneComponent.K2_GetComponentLocation` (`self.TianCanJiao`)) (`SceneComponent.K2_GetComponentLocation` (`/Game/PAP/BluePrint/BP_PawnBoat.Location Taker` _boatref_2)))) (`self.K2_GetActorRotation` _boatref_2))))
  ;[1 1 1] 往返次数
  (if (< (`self.StepTime`) 3)
    (if (`self.IsMovingDown?`)
      ;[1 1 1] 往返运动
      (`SceneComponent.K2_AddWorldOffset` (`self.TianCanJiao`) _returnvalue_3 false false)
      (set `self.CurrentMoveDistance` (- (`self.CurrentMoveDistance`) (`KismetMathLibrary.VSize` _returnvalue_3)))
      (if (< (`self.CurrentMoveDistance`) (`self.StepDepth`))
        (set `self.IsMovingDown?` false)
        (`/Engine/EditorBlueprintResources/StandardMacros.IncrementInt` (`self.StepTime`)))
      (else
        (`SceneComponent.K2_AddWorldOffset` (`self.TianCanJiao`) _returnvalue_2 false false)
        (set `self.CurrentMoveDistance` (+ (`self.CurrentMoveDistance`) (`KismetMathLibrary.VSize` _returnvalue_2)))
        (if (> (`self.CurrentMoveDistance`) 0.0)
          (set `self.IsMovingDown?` true))))
    (elif (> _tiancanjiaocount 0)
      ;[1 1 1] 若减引用计数后为0，则为最后一次，那么应用冲量
      (bind _result (`/Engine/EditorBlueprintResources/StandardMacros.DecrementInt` _tiancanjiaocount)
        (:`  `
          (if (== _result 0)
            (bind `_金钟罩开启_` (`/Game/PAP/BluePrint/Gift/BP_GiftManager.金钟罩开启?` (`self.GiftManagerRef`)))
            (if (not `_金钟罩开启_`)
              (set `/Game/PAP/BluePrint/BP_PawnBoat.Velocity` (* (`self.StepForce`) (`KismetMathLibrary.MakeVector` _returnvalue_x _returnvalue_y)) (`self.BoatRef`))
              (`KismetSystemLibrary.PrintString` "Hello")
              (set `self.ABS_X` 0.0 :!label _label)
              (set `self.ABS_Y` 0.0)
              (if (> (`KismetMathLibrary.Abs` _returnvalue_y_2) (`KismetMathLibrary.Abs` _returnvalue_x_2))
                _
                (elif (< _returnvalue_x_2 0.0)
                  (set `/Game/PAP/BluePrint/BP_PawnBoat.SwayVelocity` (- _swayvelocity _swayimpuse) _boatref)
                  (else
                    (set `/Game/PAP/BluePrint/BP_PawnBoat.SwayVelocity` (+ _swayvelocity _swayimpuse) _boatref)))))
            (else
              (goto _label)))
          (`self.K2_DestroyActor`))))))

(fn `UserConstructionScript`)