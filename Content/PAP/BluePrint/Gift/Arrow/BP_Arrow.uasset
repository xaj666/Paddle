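; Gift arrow projectile that homes in on a randomly chosen left or right skeleton on BP_PawnBoat and knocks the boat along.
; Tick moves it toward the target and box-traces, setting boat velocity from the direction cached at spawn.
; On a matching component tag it becomes an instance in that side's HISM, registers the index with BP_GiftManager's timer maps, then destroys itself.
; The Hit-event collision approach is left disconnected.
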(event `self.ReceiveBeginPlay`
  (bind _boatref (`self.BoatRef`))
  (`|ExecutionSequence`
    (:`then_0`
      (bind _returnvalue (`GameplayStatics.GetActorOfClass` "/Game/PAP/BluePrint/BP_PawnBoat.BP_PawnBoat_C"))
      (bind _output_get (set `self.BoatRef` _returnvalue))
      (bind _returnvalue_2 (`GameplayStatics.GetActorOfClass` "/Game/PAP/BluePrint/Gift/BP_GiftManager.BP_GiftManager_C"))
      (bind _output_get_2 (set `self.GiftManager` _returnvalue_2)))
    (:`then_1`
      (set `self.ArrowDirection` (`KismetMathLibrary.Normal` (- (`SceneComponent.K2_GetComponentLocation` (`/Game/PAP/BluePrint/BP_PawnBoat.Location Taker` _output_get)) (`SceneComponent.K2_GetComponentLocation` (`self.Arrow`)))))
      (set `self.BoneName` "Spine_03")
      (bind _output_get_3 (set `self.Left?` (`KismetMathLibrary.RandomBool`)))
      (if _output_get_3
        (set `self.Target Skeleton` (`/Game/PAP/BluePrint/BP_PawnBoat.Skeleton_L_Display` _boatref))
        (else
          (set `self.Target Skeleton` (`/Game/PAP/BluePrint/BP_PawnBoat.Skeleton_R_Display` _boatref)))))))

(event `self.ReceiveTick`
  (params (DeltaSeconds :type "Float (single-precision)"))
  (bind _arrow (`self.Arrow`))
  (bind _giftmanager (`self.GiftManager`))
  (bind _giftmanager_2 (`self.GiftManager`))
  (bind _returnvalue (`SceneComponent.K2_GetComponentLocation` _arrow))
  (bind _returnvalue_2 (`SceneComponent.K2_GetComponentToWorld` (`self.Arrow`)))
  (bind _returnvalue_3 (`SceneComponent.K2_GetComponentLocation` (`self.Arrow`)))
  (bind _returnvalue_4 (`SceneComponent.K2_GetComponentLocation` (`self.Target Skeleton`)))
  ;[1 1 1] Tick : 盒体检测方案
  (if (`self.NotHitYet?`)
    (`SceneComponent.K2_AddWorldOffset` _arrow (* (`KismetMathLibrary.Normal` (- _returnvalue_4 _returnvalue_3)) 20.0) false false)
    (`SceneComponent.K2_SetWorldRotation` _arrow (`KismetMathLibrary.FindLookAtRotation` _returnvalue_3 _returnvalue_4) false false)
    (bind (_outhit _returnvalue_5) (`KismetSystemLibrary.BoxTraceSingleForObjects` :`Start` _returnvalue :`End` _returnvalue :`HalfSize` (3.0 3.0 3.0) :`ObjectTypes` (`self.Object Types`) :`bTraceComplex` true :`DrawTime` 1.0))
    (if _returnvalue_5
      (bind (_bblockinghit _binitialoverlap _time _distance _location _impactpoint _normal _impactnormal _physmat _hitactor _hitcomponent) (`GameplayStatics.BreakHitResult` _outhit))
      (cast `/Game/PAP/BluePrint/BP_PawnBoat` _hitactor)
      (set `/Game/PAP/BluePrint/BP_PawnBoat.Velocity` (* (`self.ArrowDirection`) 300.0) (`self.BoatRef`))
      (if (`self.Left?`)
        (if (`ActorComponent.ComponentHasTag` _hitcomponent "L")
          (bind _returnvalue_6 (`InstancedStaticMeshComponent.AddInstance` (`/Game/PAP/BluePrint/BP_PawnBoat.ArrowHISM_L` (`self.BoatRef`)) _returnvalue_2 true))
          (`BlueprintMapLibrary.Map_Add` (`/Game/PAP/BluePrint/Gift/BP_GiftManager.LHISMIndex-Timer_Map` _giftmanager_2) _returnvalue_6)
          (`KismetArrayLibrary.Array_Add` (`/Game/PAP/BluePrint/Gift/BP_GiftManager.LHISMIndex` _giftmanager_2) _returnvalue_6)
          (set `self.NotHitYet?` false :!label _label)
          (`KismetSystemLibrary.Delay` 0.2)
          (`self.K2_DestroyActor`))
        (elif (`ActorComponent.ComponentHasTag` _hitcomponent "Character")
          (bind _returnvalue_7 (`InstancedStaticMeshComponent.AddInstance` (`/Game/PAP/BluePrint/BP_PawnBoat.ArrowHISM_R` (`self.BoatRef`)) _returnvalue_2 true))
          (`BlueprintMapLibrary.Map_Add` (`/Game/PAP/BluePrint/Gift/BP_GiftManager.RHISMIndex-Timer_Map` _giftmanager) _returnvalue_7)
          (`KismetArrayLibrary.Array_Add` (`/Game/PAP/BluePrint/Gift/BP_GiftManager.RHISMIndex` _giftmanager) _returnvalue_7)
          (goto _label))))))

(event `self.ReceiveHit`
  (params (MyComp :type "PrimitiveComponent Object Reference") (Other :type "Actor Object Reference") (OtherComp :type "PrimitiveComponent Object Reference") (bSelfMoved :type Boolean) (HitLocation :type "Vector Structure") (HitNormal :type "Vector Structure") (NormalImpulse :type "Vector Structure") (Hit :type "HitResult Structure (by ref)")))

(fn `UserConstructionScript`)