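; Arrow instance container actor that renders arrows through a Hierarchical Instanced Static Mesh, working with BP_GiftManager.
; AddShowInstance always adds a new instance; hiding updates the instance's transform and records its index in HiddenInstanceArray.
; GetHiddenInstance pops the oldest hidden index or returns -1, but the reuse nodes in AddShowInstance are disconnected.
; When the hidden array reaches 100 entries, the actor removes itself from the manager's list and destroys itself.
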(event `self.ReceiveBeginPlay`
  (bind _returnvalue (`GameplayStatics.GetActorOfClass` "/Game/PAP/BluePrint/Gift/BP_GiftManager.BP_GiftManager_C"))
  (set `self.GiftManagerRef` _returnvalue))

(fn `Add / Show Instance`
  (params (`Arrow Trans` :type "Transform Structure"))
  (locals (Trans :type "Transform Structure"))
  (`InstancedStaticMeshComponent.AddInstance` (`self.HierarchicalInstancedStaticMesh`) `Arrow Trans` false))

(fn `GetHiddenInstance`
  (returns (Output_Get :type Integer))
  (locals (`ISM Index` :type Integer))
  (if (`KismetArrayLibrary.Array_IsNotEmpty` (`self.HiddenInstanceArray`))
    (bind _output_get (set `local.ISM Index` (`|GetArrayItem` (`self.HiddenInstanceArray`))))
    (`KismetArrayLibrary.Array_Remove` (`self.HiddenInstanceArray`))
    (else
      (set `local.ISM Index` -1)))
  (return _output_get))

(fn `Hide Instance`
  (params (Index :type Integer))
  (`InstancedStaticMeshComponent.UpdateInstanceTransform` (`self.HierarchicalInstancedStaticMesh`) Index (`KismetMathLibrary.MakeTransform` (0.0 0.0 0.0)) true false false)
  (bind _returnvalue (`KismetArrayLibrary.Array_Add` (`self.HiddenInstanceArray`) Index))
  (`KismetSystemLibrary.PrintString` (`KismetStringLibrary.Concat_StrStr` "NO." (`KismetStringLibrary.Conv_IntToString` Index) "Arrow filled into slot " (`KismetStringLibrary.Conv_IntToString` _returnvalue)))
  (if (== _returnvalue 99)
    (`/Game/PAP/BluePrint/Gift/BP_GiftManager.RemoveHISM FromList` (`self.GiftManagerRef`) self)
    (`KismetSystemLibrary.PrintString` "Fulled HISM Destried" true true (struct :`R` 1.0 :`G` 0.289607 :`B` 0.259757 :`A` 1.0) 5.0)
    (`self.K2_DestroyActor`)))

(fn `UserConstructionScript`)