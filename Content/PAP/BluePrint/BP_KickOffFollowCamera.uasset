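; Temporary kick-off camera that tracks one of the two skeleton characters on the player's boat pawn.
; On BeginPlay it takes both skeleton display references from BP_PawnBoat, becomes the first player's view target, and destroys itself after a short delay.
; Each tick it rotates its camera component to look at the left or right skeleton, chosen by the FollowLeftCharacter flag.
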(event `self.ReceiveBeginPlay`
  (`|ExecutionSequence`
    (:`then_0`
      (bind _returnvalue (`GameplayStatics.GetActorOfClass` "/Game/PAP/BluePrint/BP_PawnBoat.BP_PawnBoat_C"))
      (set `self.Skeleton L Display` (`/Game/PAP/BluePrint/BP_PawnBoat.Skeleton_L_Display` _returnvalue))
      (set `self.Skeleton R Display` (`/Game/PAP/BluePrint/BP_PawnBoat.Skeleton_R_Display` _returnvalue))
      (`PlayerController.SetViewTargetWithBlend` (`PlayerState.GetPlayerController` (`GameplayStatics.GetPlayerState` 0)) self 0.0 "VTBlend_Linear" 0.0 false))
    (:`then_1`
      (`KismetSystemLibrary.Delay` 2.0)
      (`self.K2_DestroyActor`))))

(event `self.ReceiveTick`
  (params (DeltaSeconds :type "Float (single-precision)"))
  (bind _returnvalue (`SceneComponent.K2_GetComponentLocation` (`self.CameraComponent`)))
  (if (`self.FollowLeftCharacter?`)
    (`SceneComponent.K2_SetWorldRotation` (`self.CameraComponent`) (`KismetMathLibrary.FindLookAtRotation` _returnvalue (`SceneComponent.K2_GetComponentLocation` (`self.Skeleton L Display`))) false false)
    (else
      (`SceneComponent.K2_SetWorldRotation` (`self.CameraComponent`) (`KismetMathLibrary.FindLookAtRotation` _returnvalue (`SceneComponent.K2_GetComponentLocation` (`self.Skeleton R Display`))) false false))))

(fn `UserConstructionScript`)