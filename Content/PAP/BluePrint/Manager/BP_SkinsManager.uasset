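; Manager actor that swaps the character and boat skins on BP_PawnBoat, caching that pawn's components on BeginPlay.
; CharacterSkinChange sets the left or right paddler's mesh, anim class and hand-tuned display and paddle transforms per anime character; the frog (蛙) skin shows a separate cloth mesh instead.
; BoatSkinChange toggles kayak or lifeboat mesh visibility by name.
; CharacterStringNameToEnum maps names to skin enums, with no frog entry.
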(event `self.ReceiveBeginPlay`
  (bind _returnvalue (`GameplayStatics.GetActorOfClass` "/Game/PAP/BluePrint/BP_PawnBoat.BP_PawnBoat_C"))
  (bind _output_get (set `self.BoatRef` _returnvalue))
  (set `self.Skeleton L Display` (`/Game/PAP/BluePrint/BP_PawnBoat.Skeleton_L_Display` _output_get))
  (set `self.Skeleton R Display` (`/Game/PAP/BluePrint/BP_PawnBoat.Skeleton_R_Display` _output_get))
  (set `self.Paddle L` (`/Game/PAP/BluePrint/BP_PawnBoat.PaddleL` _output_get))
  (set `self.Paddle R` (`/Game/PAP/BluePrint/BP_PawnBoat.PaddleR` _output_get))
  (set `self.Skeleton L Cloth` (`/Game/PAP/BluePrint/BP_PawnBoat.Skeleton_L_Cloth` _output_get))
  (set `self.Skeleton R Cloth` (`/Game/PAP/BluePrint/BP_PawnBoat.Skeleton_R_Cloth` _output_get)))

(fn `BoatSkinChange`
  (params (BoatName :type String))
  (bind _boatref (`self.BoatRef`))
  (bind _boatref_2 (`self.BoatRef`))
  (if (`KismetStringLibrary.EqualEqual_StrStr` BoatName "皮划艇")
    (`SceneComponent.SetVisibility` (`/Game/PAP/BluePrint/BP_PawnBoat.BoatMesh` _boatref_2) true false)
    (`SceneComponent.SetVisibility` (`/Game/PAP/BluePrint/BP_PawnBoat.BoatMesh_1` _boatref_2) false false)
    (elif (`KismetStringLibrary.EqualEqual_StrStr` BoatName "救生艇")
      (`SceneComponent.SetVisibility` (`/Game/PAP/BluePrint/BP_PawnBoat.BoatMesh` _boatref) false false)
      (`SceneComponent.SetVisibility` (`/Game/PAP/BluePrint/BP_PawnBoat.BoatMesh_1` _boatref) true false))))

(fn `CharacterSkinChange`
  (params (SkinEnum :type "/Game/PAP/Enum/SkinName_Enum Enum" :default "NewEnumerator0") (`Left?` :type Boolean))
  (locals (`Skin Name` :type "/Game/PAP/Enum/SkinName_Enum Enum" :default "NewEnumerator0"))
  (bind _skeleton_l_display (`self.Skeleton L Display`))
  (bind _skeleton_l_display_2 (`self.Skeleton L Display`))
  (bind _skeleton_l_display_3 (`self.Skeleton L Display`))
  (bind _skeleton_l_display_4 (`self.Skeleton L Display`))
  (bind _skeleton_l_display_5 (`self.Skeleton L Display`))
  (bind _skeleton_r_display (`self.Skeleton R Display`))
  (bind _skeleton_r_display_2 (`self.Skeleton R Display`))
  (bind _skeleton_r_display_3 (`self.Skeleton R Display`))
  (bind _skeleton_r_display_4 (`self.Skeleton R Display`))
  (bind _skeleton_r_display_5 (`self.Skeleton R Display`))
  (bind _output_get (set `local.Skin Name` SkinEnum))
  (if `Left?`
    (if (`|EnumEquality` _output_get "NewEnumerator5")
      (`SceneComponent.SetVisibility` (`self.Skeleton L Display`) false true)
      (`SceneComponent.SetVisibility` (`self.Skeleton L Cloth`) true true)
      (else
        (`SceneComponent.SetVisibility` (`self.Skeleton L Display`) true true)
        (`SceneComponent.SetVisibility` (`self.Skeleton L Cloth`) false true)))
    (switch `/Game/PAP/Enum/SkinName_Enum` (`local.Skin Name`)
      (:`NewEnumerator0`
        ;[1 1 1] 贝吉塔
        (`SkeletalMeshComponent.SetSkeletalMeshAsset` _skeleton_l_display_2 "/Game/PAP/AnimBluePrint/CharacterAssets/BeiJiTa/贝吉塔_1_.贝吉塔_1_")
        (`SkeletalMeshComponent.SetAnimInstanceClass` _skeleton_l_display_2 "/Game/PAP/AnimBluePrint/BeiJiTa_L.BeiJiTa_L_C")
        (`SceneComponent.K2_SetRelativeTransform` _skeleton_l_display_2 (`KismetMathLibrary.MakeTransform` (0.0 0.0 -0.8) (struct) (0.017 0.017 0.017)) false false)
        (`SceneComponent.K2_SetRelativeTransform` (`self.Paddle L`) (`KismetMathLibrary.MakeTransform` (-52.13452 -0.028769 27.941571) (struct :`Pitch` 3.0 :`Yaw` 10.0 :`Roll` -82.0) (0.35 0.2625 0.35)) false false))
      (:`NewEnumerator1`
        ;[1 1 1] 蓝发悟空
        (`SkeletalMeshComponent.SetSkeletalMeshAsset` _skeleton_l_display_3 "/Game/PAP/AnimBluePrint/CharacterAssets/QiLongZhu/七龙珠.七龙珠")
        (`SkeletalMeshComponent.SetAnimInstanceClass` _skeleton_l_display_3 "/Game/PAP/AnimBluePrint/LongZhu_L.LongZhu_L_C")
        (`SceneComponent.K2_SetRelativeTransform` _skeleton_l_display_3 (`KismetMathLibrary.MakeTransform` (0.0 0.0 -0.8) (struct) (0.007 0.007 0.007)) false false)
        (`SceneComponent.K2_SetRelativeTransform` (`self.Paddle L`) (`KismetMathLibrary.MakeTransform` (-121.694377 -1.763251 65.492747) (struct :`Pitch` 2.86 :`Yaw` 10.0 :`Roll` -80.0) (0.8 0.6 0.8)) false false))
      (:`NewEnumerator2`
        ;[1 1 1] 金发悟空
        (`SkeletalMeshComponent.SetSkeletalMeshAsset` _skeleton_l_display_4 "/Game/PAP/AnimBluePrint/CharacterAssets/WuKong/3悟空.3悟空")
        (`SkeletalMeshComponent.SetAnimInstanceClass` _skeleton_l_display_4 "/Game/PAP/AnimBluePrint/WuKong_L.WuKong_L_C")
        (`SceneComponent.K2_SetRelativeTransform` _skeleton_l_display_4 (`KismetMathLibrary.MakeTransform` (0.0 0.0 -0.8) (struct) (0.008 0.008 0.008)) false false)
        (`SceneComponent.K2_SetRelativeTransform` (`self.Paddle L`) (`KismetMathLibrary.MakeTransform` (-94.472461 -1.20216 68.406886) (struct :`Pitch` -7.0 :`Yaw` 8.259 :`Roll` -86.0) (0.7 0.525 0.7)) false false))
      (:`NewEnumerator3`
        ;[1 1 1] 佐助
        (`SkeletalMeshComponent.SetSkeletalMeshAsset` _skeleton_l_display_5 "/Game/PAP/AnimBluePrint/CharacterAssets/ZuoZhu/佐助.佐助")
        (`SkeletalMeshComponent.SetAnimInstanceClass` _skeleton_l_display_5 "/Game/PAP/AnimBluePrint/LongZhu_L.LongZhu_L_C")
        (`SceneComponent.K2_SetRelativeTransform` _skeleton_l_display_5 (`KismetMathLibrary.MakeTransform` (0.0 0.0 -0.8) (struct) (0.013 0.013 0.013)) false false)
        (`SceneComponent.K2_SetRelativeTransform` (`self.Paddle L`) (`KismetMathLibrary.MakeTransform` (-67.911571 -1.866624 29.805606) (struct :`Pitch` 3.0 :`Yaw` 8.95 :`Roll` -85.0) (0.45 0.3375 0.45)) false false))
      (:`NewEnumerator4`
        ;[1 1 1] 鸣人
        (`SkeletalMeshComponent.SetSkeletalMeshAsset` _skeleton_l_display "/Game/PAP/AnimBluePrint/CharacterAssets/MingRen/鸣人.鸣人")
        (`SkeletalMeshComponent.SetAnimInstanceClass` _skeleton_l_display "/Game/PAP/AnimBluePrint/LongZhu_L.LongZhu_L_C")
        (`SceneComponent.K2_SetRelativeTransform` _skeleton_l_display (`KismetMathLibrary.MakeTransform` (0.0 0.0 -0.8) (struct) (0.013 0.013 0.013)) false false)
        (`SceneComponent.K2_SetRelativeTransform` (`self.Paddle L`) (`KismetMathLibrary.MakeTransform` (-67.911571 -1.866624 29.805606) (struct :`Pitch` 3.0 :`Yaw` 8.95 :`Roll` -85.0) (0.45 0.3375 0.45)) false false)))
    (else
      (if (`|EnumEquality` (`local.Skin Name`) "NewEnumerator5")
        (`SceneComponent.SetVisibility` (`self.Skeleton R Display`) false true)
        (`SceneComponent.SetVisibility` (`self.Skeleton R Cloth`) true true)
        (else
          (`SceneComponent.SetVisibility` (`self.Skeleton R Display`) true true)
          (`SceneComponent.SetVisibility` (`self.Skeleton R Cloth`) false true)))
      (switch `/Game/PAP/Enum/SkinName_Enum` (`local.Skin Name`)
        (:`NewEnumerator0`
          ;[1 1 1] 贝吉塔
          (`SkeletalMeshComponent.SetSkeletalMeshAsset` _skeleton_r_display_4 "/Game/PAP/AnimBluePrint/CharacterAssets/BeiJiTa/贝吉塔_1_.贝吉塔_1_")
          (`SkeletalMeshComponent.SetAnimInstanceClass` _skeleton_r_display_4 "/Game/PAP/AnimBluePrint/BeiJiTa_R.BeiJiTa_R_C")
          (`SceneComponent.K2_SetRelativeTransform` _skeleton_r_display_4 (`KismetMathLibrary.MakeTransform` (0.0 0.0 -0.8) (struct) (0.017 0.017 0.017)) false false)
          (`SceneComponent.K2_SetRelativeTransform` (`self.Paddle R`) (`KismetMathLibrary.MakeTransform` (-41.503894 -5.722631 -28.812304) (struct :`Yaw` 8.84 :`Roll` 86.0) (0.35 0.2625 0.35)) false false))
        (:`NewEnumerator1`
          ;[1 1 1] 蓝发悟空
          (`SkeletalMeshComponent.SetSkeletalMeshAsset` _skeleton_r_display "/Game/PAP/AnimBluePrint/CharacterAssets/QiLongZhu/七龙珠.七龙珠")
          (`SkeletalMeshComponent.SetAnimInstanceClass` _skeleton_r_display "/Game/PAP/AnimBluePrint/LongZhu_R.LongZhu_R_C")
          (`SceneComponent.K2_SetRelativeTransform` _skeleton_r_display (`KismetMathLibrary.MakeTransform` (0.0 0.0 -0.8) (struct) (0.007 0.007 0.007)) false false)
          (`SceneComponent.K2_SetRelativeTransform` (`self.Paddle R`) (`KismetMathLibrary.MakeTransform` (-91.007139 -38.523317 -63.983295) (struct :`Pitch` -0.298 :`Yaw` 8.844 :`Roll` 104.395) (0.8 0.6 0.8)) false false))
        (:`NewEnumerator2`
          ;[1 1 1] 金发悟空
          (`SkeletalMeshComponent.SetSkeletalMeshAsset` _skeleton_r_display_2 "/Game/PAP/AnimBluePrint/CharacterAssets/WuKong/3悟空.3悟空")
          (`SkeletalMeshComponent.SetAnimInstanceClass` _skeleton_r_display_2 "/Game/PAP/AnimBluePrint/WuKong_R.WuKong_R_C")
          (`SceneComponent.K2_SetRelativeTransform` _skeleton_r_display_2 (`KismetMathLibrary.MakeTransform` (0.0 0.0 -0.8) (struct) (0.008 0.008 0.008)) false false)
          (`SceneComponent.K2_SetRelativeTransform` (`self.Paddle R`) (`KismetMathLibrary.MakeTransform` (-88.034732 -21.748145 -32.02797) (struct :`Pitch` -14.718 :`Yaw` 5.91 :`Roll` 96.37) (0.7 0.525 0.7)) false false))
        (:`NewEnumerator3`
          ;[1 1 1] 佐助
          (`SkeletalMeshComponent.SetSkeletalMeshAsset` _skeleton_r_display_3 "/Game/PAP/AnimBluePrint/CharacterAssets/ZuoZhu/佐助.佐助")
          (`SkeletalMeshComponent.SetAnimInstanceClass` _skeleton_r_display_3 "/Game/PAP/AnimBluePrint/LongZhu_R.LongZhu_R_C")
          (`SceneComponent.K2_SetRelativeTransform` _skeleton_r_display_3 (`KismetMathLibrary.MakeTransform` (0.0 0.0 -0.8) (struct) (0.013 0.013 0.013)) false false)
          (`SceneComponent.K2_SetRelativeTransform` (`self.Paddle R`) (`KismetMathLibrary.MakeTransform` (-48.291311 -16.333253 -36.605504) (struct :`Pitch` 5.16 :`Yaw` 8.1 :`Roll` 101.0) (0.45 0.3375 0.45)) false false))
        (:`NewEnumerator4`
          ;[1 1 1] 鸣人
          (`SkeletalMeshComponent.SetSkeletalMeshAsset` _skeleton_r_display_5 "/Game/PAP/AnimBluePrint/CharacterAssets/MingRen/鸣人.鸣人")
          (`SkeletalMeshComponent.SetAnimInstanceClass` _skeleton_r_display_5 "/Game/PAP/AnimBluePrint/LongZhu_R.LongZhu_R_C")
          (`SceneComponent.K2_SetRelativeTransform` _skeleton_r_display_5 (`KismetMathLibrary.MakeTransform` (0.0 0.0 -0.8) (struct) (0.013 0.013 0.013)) false false)
          (`SceneComponent.K2_SetRelativeTransform` (`self.Paddle R`) (`KismetMathLibrary.MakeTransform` (-48.291311 -16.333253 -36.605504) (struct :`Pitch` 5.16 :`Yaw` 8.1 :`Roll` 101.0) (0.45 0.3375 0.45)) false false))))))

(fn `CharacterStringNameToEnum`
  (params (StringName :type String))
  (returns (NewParam :type "/Game/PAP/Enum/SkinName_Enum Enum"))
  (locals (EnumName :type "/Game/PAP/Enum/SkinName_Enum Enum" :default "NewEnumerator0"))
  (if (`KismetStringLibrary.EqualEqual_StrStr` StringName "贝吉塔")
    (set `local.EnumName` "NewEnumerator0")
    (return (`local.EnumName`))
    (elif (`KismetStringLibrary.EqualEqual_StrStr` StringName "蓝发悟空")
      (set `local.EnumName` "NewEnumerator1")
      (return (`local.EnumName`))
      (elif (`KismetStringLibrary.EqualEqual_StrStr` StringName "金发悟空")
        (set `local.EnumName` "NewEnumerator2")
        (return (`local.EnumName`))
        (elif (`KismetStringLibrary.EqualEqual_StrStr` StringName "佐助")
          (set `local.EnumName` "NewEnumerator3")
          (return (`local.EnumName`))
          (elif (`KismetStringLibrary.EqualEqual_StrStr` StringName "鸣人")
            (set `local.EnumName` "NewEnumerator4")
            (return (`local.EnumName`))))))))

(fn `UserConstructionScript`)