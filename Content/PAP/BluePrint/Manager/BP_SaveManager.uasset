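; BP_SaveManager is an actor that provides the game's saved settings and the effect sound volume derived from them.
; GetSaveData loads the SettingsData slot on each call, or creates and saves a new one if none exists, and caches it in SaveSettingsData.
; GetEffectMusic calls it and multiplies total by effect volume, scaled down by 10000; an invalid save only prints a warning.
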(fn `GetEffectMusic`
  (returns (`ReturnTotal - EffectMusic` :type "Float (double-precision)"))
  (bind _save_settingsdata1 (`self.GetSaveData`))
  (`/Engine/EditorBlueprintResources/StandardMacros.IsValid` _save_settingsdata1
    (:`Is Valid`
      _)
    (:`Is Not Valid`
      (`KismetSystemLibrary.PrintString` "Get Effect Music : SaveSettingsData is Invalid")))
  (bind (_sounddata_totalsoundvalue _sounddata_effectsoundvalue) (break `/Game/PAP/UI/ConfigData/Structures/SoundData` (`/Game/PAP/UI/ConfigData/SettingsData.SoundData` _save_settingsdata1)))
  (return (/ (* _sounddata_totalsoundvalue _sounddata_effectsoundvalue) 10000.0)))

(fn `GetSaveData`
  (returns (Save_SettingsData1 :type "/Game/PAP/UI/ConfigData/SettingsData Object Reference"))
  (locals (Save_SettingsData :type "/Game/PAP/UI/ConfigData/SettingsData Object Reference"))
  (`KismetSystemLibrary.PrintString` "SaveDataFuncCalled")
  (bind _returnvalue (`GameplayStatics.DoesSaveGameExist` "SettingsData"))
  (if _returnvalue
    (bind _returnvalue_2 (`GameplayStatics.LoadGameFromSlot` "SettingsData"))
    (bind _assettings_data (cast `/Game/PAP/UI/ConfigData/SettingsData` _returnvalue_2))
    (set `local.Save_SettingsData` _assettings_data)
    (else
      (bind _returnvalue_3 (`GameplayStatics.CreateSaveGameObject` "/Game/PAP/UI/ConfigData/SettingsData.SettingsData_C"))
      (bind _output_get (set `local.Save_SettingsData` _returnvalue_3))
      (`GameplayStatics.SaveGameToSlot` _output_get "SettingsData")))
  (return (`local.Save_SettingsData`)))

(fn `UserConstructionScript`)