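; Manager actor that drives all BP_CannonBall actors in the level as looping projectiles with randomized pauses between shots.
; BeginPlay caches the cannonballs; Tick moves each ball, flame particle and sphere along rotated forward vectors once its delay expires.
; Beyond the maximum distance from its start, ball and particle snap back to their stored start locations and get a new random delay.
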(event `self.ReceiveBeginPlay`
  (bind _outactors (`GameplayStatics.GetAllActorsOfClass` "/Game/PAP/BluePrint/Mechanics/Obstacle/Dynamic/BP_CannonBall.BP_CannonBall_C"))
  (bind _output_get (set `self.CannonBallsRef` _outactors))
  (for _ _output_get
    _))

(event `self.ReceiveTick`
  (params (DeltaSeconds :type "Float (single-precision)"))
  (bind _ballref (`self.BallRef`))
  (bind _ballref_2 (`self.BallRef`))
  (bind _ballref_3 (`self.BallRef`))
  (bind _ballref_4 (`self.BallRef`))
  (bind _cannonball (`/Game/PAP/BluePrint/Mechanics/Obstacle/Dynamic/BP_CannonBall.CannonBall` (`self.BallRef`)))
  (bind _p_flamethrower (`/Game/PAP/BluePrint/Mechanics/Obstacle/Dynamic/BP_CannonBall.P_Flamethrower` (`self.BallRef`)))
  (bind _returnvalue (* (* (`KismetMathLibrary.GreaterGreater_VectorRotator` (`SceneComponent.GetForwardVector` _cannonball) (struct :`Yaw` 90.0)) (`self.CannonBallSpeed`)) (`self.Delta Seconds`)))
  (bind _returnvalue_2 (+ (`SceneComponent.K2_GetComponentLocation` _p_flamethrower) (* (* (`KismetMathLibrary.GreaterGreater_VectorRotator` (`SceneComponent.GetForwardVector` _p_flamethrower) (struct :`Yaw` 180.0)) (`self.CannonBallSpeed`)) (`self.Delta Seconds`))))
  (set `self.Delta Seconds` DeltaSeconds)
  (for _array_element (`self.CannonBallsRef`)
    (set `self.BallRef` _array_element)
    (if (> (`KismetMathLibrary.VSize` (`KismetMathLibrary.Vector_GetAbs` (- (`SceneComponent.K2_GetComponentLocation` (`/Game/PAP/BluePrint/Mechanics/Obstacle/Dynamic/BP_CannonBall.CannonBall` _ballref)) (`/Game/PAP/BluePrint/Mechanics/Obstacle/Dynamic/BP_CannonBall.BallStartLoc` _ballref)))) (`self.MaxMoveDistance`))
      ;[1 1 1] 位置回溯
      (`SceneComponent.K2_SetWorldLocation` (`/Game/PAP/BluePrint/Mechanics/Obstacle/Dynamic/BP_CannonBall.CannonBall` _ballref_3) (`/Game/PAP/BluePrint/Mechanics/Obstacle/Dynamic/BP_CannonBall.BallStartLoc` _ballref_3) false false)
      (`SceneComponent.K2_SetWorldLocation` (`/Game/PAP/BluePrint/Mechanics/Obstacle/Dynamic/BP_CannonBall.P_Flamethrower` _ballref_3) (`/Game/PAP/BluePrint/Mechanics/Obstacle/Dynamic/BP_CannonBall.ParticleStartLoc` _ballref_3) false false)
      ;[1 1 1] 随机CD
      (set `/Game/PAP/BluePrint/Mechanics/Obstacle/Dynamic/BP_CannonBall.DelayTime` (`KismetMathLibrary.RandomFloatInRange` 0.5 5.0) (`self.BallRef`))
      ;[1 1 1] 清空已移动距离
      (set `/Game/PAP/BluePrint/Mechanics/Obstacle/Dynamic/BP_CannonBall.MovedDistance` 0.0 (`self.BallRef`))
      (elif (< (`/Game/PAP/BluePrint/Mechanics/Obstacle/Dynamic/BP_CannonBall.DelayTime` (`self.BallRef`)) 0.0)
        ;[1 1 1] Move
        (`SceneComponent.K2_SetWorldLocation` _cannonball (+ (`SceneComponent.K2_GetComponentLocation` _cannonball) _returnvalue) false false)
        (`SceneComponent.K2_SetWorldLocation` _p_flamethrower _returnvalue_2 false false)
        (`SceneComponent.K2_SetWorldLocation` (`/Game/PAP/BluePrint/Mechanics/Obstacle/Dynamic/BP_CannonBall.Sphere` (`self.BallRef`)) _returnvalue_2 false false)
        ;[1 1 1] 更新已移动距离
        (set `/Game/PAP/BluePrint/Mechanics/Obstacle/Dynamic/BP_CannonBall.MovedDistance` (+ (`/Game/PAP/BluePrint/Mechanics/Obstacle/Dynamic/BP_CannonBall.MovedDistance` _ballref_2) (`KismetMathLibrary.VSize` _returnvalue)) _ballref_2)
        (else
          ;[1 1 1] 更新CD
          (set `/Game/PAP/BluePrint/Mechanics/Obstacle/Dynamic/BP_CannonBall.DelayTime` (- (`/Game/PAP/BluePrint/Mechanics/Obstacle/Dynamic/BP_CannonBall.DelayTime` _ballref_4) (`self.Delta Seconds`)) _ballref_4))))))

(fn `UserConstructionScript`)