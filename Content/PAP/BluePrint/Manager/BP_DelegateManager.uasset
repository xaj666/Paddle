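; BP_DelegateManager is a hub actor that binds gameplay delegates and routes them to the main HUD widget, the player boat and the gift manager.
; After a short BeginPlay delay it caches those references, then forwards menu toggles to MainUI and checkpoint hits to the boat.
; Death plays an explosion and random sound, respawns the boat above its last checkpoint, and optionally resets its size through GiftManager.
; The animation and beach-ball handlers are empty.
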(event `self.ReceiveBeginPlay`
  (`KismetSystemLibrary.Delay` 0.1)
  ;[1 1 1] 初始化引用
  (`|ExecutionSequence`
    (:`then_0`
      (bind _aspap_hud (cast `/Game/PAP/UI/PAP_HUD` (`PlayerController.GetHUD` (`GameplayStatics.GetPlayerController` 0))))
      (bind _mainui (`/Game/PAP/UI/PAP_HUD.MainUI` _aspap_hud))
      (set `self.Main UI` _mainui)
      (set `self.Meme Hot Bar Ref` (`/Game/PAP/UI/UI_MainScreen.MemeHotBarRef` _mainui)))
    (:`then_1`
      (bind _returnvalue (`GameplayStatics.GetActorOfClass` "/Game/PAP/BluePrint/BP_PawnBoat.BP_PawnBoat_C"))
      (set `self.BoatRef` _returnvalue)
      (`|ExecutionSequence`
        (:`then_0`
          ;[1 1 1] 表情包菜单代理绑定
          (add `self.OnToggleMemePlate` (delegate `OnToggleMemePlate_Event`))
          ;[1 1 1] 整蛊动作菜单代理绑定
          (add `self.On Toggle Anim Plate` (delegate `OnToggleAnimPlate_Event`))
          (add `self.OnToggleSettingsPlate` (delegate `OnToggleSettingsPlate_Event`)))
        (:`then_1`
          ;[1 1 1] Death
          (add `self.OnDeath` (delegate `OnDeath_Event`)))
        (:`then_2`
          ;[1 1 1] 检查点碰撞
          (add `self.OnCheckPointHits` (delegate `OnCheckPointHits_Event`))
          (add `self.OnAnimPlay` (delegate `On Anim Play_Event`)))
        (:`then_3`
          (add `self.OnBeachBallOverlap` (delegate `OnBeachBallOverlap_Event`)))))
    (:`then_2`
      (bind _returnvalue_2 (`GameplayStatics.GetActorOfClass` "/Game/PAP/BluePrint/Gift/BP_GiftManager.BP_GiftManager_C"))
      (set `self.GiftManager Ref` _returnvalue_2))))

(event `OnToggleMemePlate_Event`
  ;[1 1 1] 表情包菜单代理绑定
  (`/Game/PAP/UI/UI_MainScreen.ToggleMemePlate` (`self.Main UI`)))

(event `OnToggleAnimPlate_Event` :!signature `self.On Toggle Anim Plate`
  (params (`OpenAnimPlate?` :type Boolean))
  ;[1 1 1] 整蛊动作菜单代理绑定
  (`/Game/PAP/UI/UI_MainScreen.ToggleAnimPlate` (`self.Main UI`) `OpenAnimPlate?`))

(event `OnToggleSettingsPlate_Event` :!signature `self.OnToggleSettingsPlate`
  (params (`Open Settings Plate?` :type Boolean))
  (`/Game/PAP/UI/UI_MainScreen.Toggle Settings Plate` (`self.Main UI`) `Open Settings Plate?`))

(event `OnDeath_Event`
  (bind _boatref (`self.BoatRef`))
  (bind _boatref_2 (`self.BoatRef`))
  (bind (_lastcheckpointloc_x _lastcheckpointloc_y _lastcheckpointloc_z) (`KismetMathLibrary.BreakVector` (`/Game/PAP/BluePrint/BP_PawnBoat.LastCheckPointLoc` _boatref)))
  ;[1 1 1] Death
  (`NiagaraFunctionLibrary.SpawnSystemAtLocation` "/Game/Death_SE/FX/NS_Explosion05.NS_Explosion05" (`SceneComponent.K2_GetComponentLocation` (`/Game/PAP/BluePrint/BP_PawnBoat.Location Taker` (`self.BoatRef`))))
  (`self.RandomDeathSound`)
  (set `/Game/PAP/BluePrint/BP_PawnBoat.IsAlive?` false _boatref_2)
  (set `/Game/PAP/BluePrint/BP_PawnBoat.Velocity` (0.0 0.0 0.0) _boatref_2)
  (`PrimitiveComponent.SetCollisionEnabled` (`/Game/PAP/BluePrint/BP_PawnBoat.Location Taker` _boatref) "NoCollision")
  (`self.SetActorHiddenInGame` _boatref true)
  (`KismetSystemLibrary.Delay` 0.5)
  (`SceneComponent.K2_SetWorldLocation` (`/Game/PAP/BluePrint/BP_PawnBoat.Location Taker` _boatref) (`KismetMathLibrary.MakeVector` _lastcheckpointloc_x _lastcheckpointloc_y (+ _lastcheckpointloc_z 30.0)) false false)
  (`self.SetActorHiddenInGame` _boatref false)
  (`PrimitiveComponent.SetCollisionEnabled` (`/Game/PAP/BluePrint/BP_PawnBoat.Location Taker` (`self.BoatRef`)) "QueryAndPhysics")
  (set `/Game/PAP/BluePrint/BP_PawnBoat.IsAlive?` true (`self.BoatRef`))
  (if (`self.死亡后大小重置？`)
    ;[1 1 1] 死亡后大小重置
    (`/Game/PAP/BluePrint/Gift/BP_GiftManager.大小重置` (`self.GiftManager Ref`) false)))

(event `OnCheckPointHits_Event` :!signature `self.OnCheckPointHits`
  (params (CheckPointLoc :type "Vector Structure"))
  ;[1 1 1] 检查点碰撞
  (`/Game/PAP/BluePrint/BP_PawnBoat.OnCheckPointHits` (`self.BoatRef`) CheckPointLoc))

(event `On Anim Play_Event`)

(event `OnBeachBallOverlap_Event` :!signature `self.OnBeachBallOverlap`
  (params (BounceDir :type "Vector Structure")))

(fn `RandomDeathSound`
  (locals (RandomIndex :type Integer :default 0))
  (bind _output_get (set `local.RandomIndex` (`KismetMathLibrary.RandomInteger` 3)))
  (if (== _output_get 0)
    (`AddComponent|NODE_AddAudioComponent-0`)
    (elif (== (`local.RandomIndex`) 1)
      (`AddComponent|NODE_AddAudioComponent-1`)
      (elif (== (`local.RandomIndex`) 2)
        (`AddComponent|NODE_AddAudioComponent-2`)))))

(fn `UserConstructionScript`)