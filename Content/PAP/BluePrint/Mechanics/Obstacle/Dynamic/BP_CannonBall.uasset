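; BP_CannonBall is a cannonball obstacle that triggers death when it hits a living player boat.
; Its sphere overlap filters for BP_PawnBoat's "BoatBody"-tagged component, then adds an audio component and, after a short delay, calls CallOnDeath on BP_DelegateManager.
; BeginPlay caches the ball and flamethrower particle start locations, which this graph never reads; no movement logic is present, and a debug print remains.
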(event `self.ReceiveBeginPlay`
  (set `self.BallStartLoc` (`SceneComponent.K2_GetComponentLocation` (`self.CannonBall`)))
  (set `self.ParticleStartLoc` (`SceneComponent.K2_GetComponentLocation` (`self.P_Flamethrower`))))

(event `self.Sphere.OnComponentBeginOverlap`
  (params (OverlappedComponent :type "PrimitiveComponent Object Reference") (OtherActor :type "Actor Object Reference") (OtherComp :type "PrimitiveComponent Object Reference") (OtherBodyIndex :type Integer) (bFromSweep :type Boolean) (SweepResult :type "HitResult Structure (by ref)"))
  (bind _asbp_pawn_boat (cast `/Game/PAP/BluePrint/BP_PawnBoat` OtherActor))
  (if (`ActorComponent.ComponentHasTag` OtherComp "BoatBody")
    (if (`/Game/PAP/BluePrint/BP_PawnBoat.IsAlive?` _asbp_pawn_boat)
      (bind _returnvalue (`GameplayStatics.GetActorOfClass` "/Game/PAP/BluePrint/Manager/BP_DelegateManager.BP_DelegateManager_C"))
      (`AddComponent|NODE_AddAudioComponent-0`)
      (`KismetSystemLibrary.Delay` 0.2)
      (`/Game/PAP/BluePrint/Manager/BP_DelegateManager.OnDeath` _returnvalue)
      (`KismetSystemLibrary.PrintString` "Hello"))))

(fn `UserConstructionScript`)