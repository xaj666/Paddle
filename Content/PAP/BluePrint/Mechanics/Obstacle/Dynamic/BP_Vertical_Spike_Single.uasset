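; A single vertical spike dynamic obstacle that keeps its collision and bounce components aligned with its animated skeleton.
; Each Tick, after the parent's logic, it snaps BoxCollision, BounceDir and Cube to the Obstacle's end bone in world space, using a fixed downward offset and rotation correction.
; BeginPlay and construction only call the parent, and the overlap event is disabled, so this Blueprint adds no hit logic of its own.
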(event `self.ReceiveBeginPlay`
  (`parent.ReceiveBeginPlay`))

(event `self.ReceiveTick`
  (params (DeltaSeconds :type "Float (single-precision)"))
  (bind (_returnvalue_location _returnvalue_rotation) (`KismetMathLibrary.BreakTransform` (`SkinnedMeshComponent.GetBoneTransform` (`self.Obstacle`) "骨骼_end" "RTS_World")))
  (bind _returnvalue (`KismetMathLibrary.ComposeRotators` (struct :`Pitch` 90.0 :`Yaw` 90.0) _returnvalue_rotation))
  (bind _returnvalue_2 (+ _returnvalue_location (0.0 0.0 -120.0)))
  (`parent.ReceiveTick` DeltaSeconds)
  (`|ExecutionSequence`
    (:`then_0`
      (`SceneComponent.K2_SetWorldLocationAndRotation` (`self.BoxCollision`) _returnvalue_2 _returnvalue false false))
    (:`then_1`
      (`SceneComponent.K2_SetWorldLocationAndRotation` (`self.BounceDir`) _returnvalue_2 _returnvalue false false))
    (:`then_2`
      (`SceneComponent.K2_SetWorldLocationAndRotation` (`self.Cube`) _returnvalue_2 _returnvalue false false))))

(fn `UserConstructionScript`
  (`parent.UserConstructionScript`))