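; BP_BoostPad is a pad that boosts player boat pawns passing over it.
; On BeginPlay it caches the forward vector of its BounceDir component as the boost direction.
; While active, its box collision checks overlaps for a BP_PawnBoat component tagged BoatBody, then passes the direction and boost force to the boat and adds two audio components.
; The boat handles the boost itself, as the pad's own impulse node is unconnected.
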(event `self.ReceiveBeginPlay`
  (`parent.ReceiveBeginPlay`)
  (set `self.Bounce Direction` (`SceneComponent.GetForwardVector` (`self.BounceDir`))))

(event `self.BoxCollision.OnComponentBeginOverlap`
  (params (OverlappedComponent :type "PrimitiveComponent Object Reference") (OtherActor :type "Actor Object Reference") (OtherComp :type "PrimitiveComponent Object Reference") (OtherBodyIndex :type Integer) (bFromSweep :type Boolean) (SweepResult :type "HitResult Structure (by ref)"))
  (if (`self.IsActive`)
    (bind _asbp_pawn_boat (cast `/Game/PAP/BluePrint/BP_PawnBoat` OtherActor))
    (if (`ActorComponent.ComponentHasTag` OtherComp "BoatBody")
      (`/Game/PAP/BluePrint/BP_PawnBoat.OnBoostPadCollisionHits` _asbp_pawn_boat (`self.Bounce Direction`) (`self.Boost Force`))
      (`AddComponent|NODE_AddAudioComponent-2`)
      (`AddComponent|NODE_AddAudioComponent-3`))))

(fn `UserConstructionScript`
  (`parent.UserConstructionScript`))