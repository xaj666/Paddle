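; BP_CheckPoint is a waypoint checkpoint that triggers when the player boat's tagged body overlaps its collision sphere.
; On a hit it reports its mesh location through BP_DelegateManager, adds an audio component and removes its UI widget, found in the GameInstance's checkpoint map.
; It then hides and deactivates, reappearing re-triggerable after a short delay, though the removed widget is not restored here.
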(event `self.ReceiveBeginPlay`
  (bind _aspap_game_instance (cast `/Game/PAP/BluePrint/PAP_GameInstance` (`GameplayStatics.GetGameInstance`)))
  (set `self.UI Check Point Map` (`/Game/PAP/BluePrint/PAP_GameInstance.UI_CheckPoint_Map` _aspap_game_instance)))

(event `self.SphereCollision.OnComponentBeginOverlap`
  (params (OverlappedComponent :type "PrimitiveComponent Object Reference") (OtherActor :type "Actor Object Reference") (OtherComp :type "PrimitiveComponent Object Reference") (OtherBodyIndex :type Integer) (bFromSweep :type Boolean) (SweepResult :type "HitResult Structure (by ref)"))
  (bind _value (`BlueprintMapLibrary.Map_Find` (`self.UI Check Point Map`) self))
  (cast `/Game/PAP/BluePrint/BP_PawnBoat` OtherActor)
  (if (`ActorComponent.ComponentHasTag` OtherComp "BoatBody")
    (if (`self.IsActivated?`)
      (set `self.IsActivated?` false)
      (bind _returnvalue (`GameplayStatics.GetActorOfClass` "/Game/PAP/BluePrint/Manager/BP_DelegateManager.BP_DelegateManager_C"))
      (`/Game/PAP/BluePrint/Manager/BP_DelegateManager.OnCheckPointHits` _returnvalue (`SceneComponent.K2_GetComponentLocation` (`self.StaticMesh`)))
      ;[1 1 1] 销毁
      (`AddComponent|NODE_AddAudioComponent-0`)
      (`/Engine/EditorBlueprintResources/StandardMacros.IsValid` _value
        (:`Is Valid`
          (`Widget.RemoveFromParent` _value))
        (:`Is Not Valid`
          _))
      (`SceneComponent.SetVisibility` (`self.DefaultSceneRoot`) false true)
      ;;[1 1 1] 5s后可重新触发
      (`KismetSystemLibrary.Delay` 5.0)
      (set `self.IsActivated?` true)
      (`SceneComponent.SetVisibility` (`self.DefaultSceneRoot`) true true))))

(fn `UserConstructionScript`
  (`parent.UserConstructionScript`))