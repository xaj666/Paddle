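; BP_BounceInvisibleWall is an invisible boundary that bounces player boats (BP_PawnBoat) back in a fixed direction.
; On BeginPlay it caches the Arrow component's forward vector as the bounce direction.
; Outer and inner box overlaps filter for components tagged BoatBody and call CallOnInvisiWallHits on the boat, each with its own force.
; Debug prints mark which layer triggered.
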(event `self.ReceiveBeginPlay`
  (set `self.BounceDirection` (`SceneComponent.GetForwardVector` (`self.Arrow`))))

(event `self.OuterBox.OnComponentBeginOverlap`
  (params (OverlappedComponent :type "PrimitiveComponent Object Reference") (OtherActor :type "Actor Object Reference") (OtherComp :type "PrimitiveComponent Object Reference") (OtherBodyIndex :type Integer) (bFromSweep :type Boolean) (SweepResult :type "HitResult Structure (by ref)"))
  (if true
    (bind _asbp_pawn_boat (cast `/Game/PAP/BluePrint/BP_PawnBoat` OtherActor))
    (if (`ActorComponent.ComponentHasTag` OtherComp "BoatBody")
      (`/Game/PAP/BluePrint/BP_PawnBoat.OnInvisiWallHits` _asbp_pawn_boat (`self.BounceDirection`) (`self.BounceForce`))
      (`KismetSystemLibrary.PrintString` "OuterTriggered" true true (struct :`R` 0.213835 :`G` 1.0 :`B` 0.240111 :`A` 1.0)))))

(event `self.OuterBox.OnComponentEndOverlap`
  (params (OverlappedComponent :type "PrimitiveComponent Object Reference") (OtherActor :type "Actor Object Reference") (OtherComp :type "PrimitiveComponent Object Reference") (OtherBodyIndex :type Integer)))

(event `self.InnerBox.OnComponentBeginOverlap`
  (params (OverlappedComponent :type "PrimitiveComponent Object Reference") (OtherActor :type "Actor Object Reference") (OtherComp :type "PrimitiveComponent Object Reference") (OtherBodyIndex :type Integer) (bFromSweep :type Boolean) (SweepResult :type "HitResult Structure (by ref)"))
  (if true
    (bind _asbp_pawn_boat (cast `/Game/PAP/BluePrint/BP_PawnBoat` OtherActor))
    (if (`ActorComponent.ComponentHasTag` OtherComp "BoatBody")
      (`/Game/PAP/BluePrint/BP_PawnBoat.OnInvisiWallHits` _asbp_pawn_boat (`self.BounceDirection`) (`self.InnerBounceForce`))
      (`KismetSystemLibrary.PrintString` "InnerTriggered" true true (struct :`R` 1.0 :`G` 0.333919 :`B` 0.244163 :`A` 1.0)))))

(fn `UserConstructionScript`)